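; Player character Blueprint for Potitt that supplies animation, UI and visual feedback for movement, combat, grappling and health.
; Gameplay events play montages, drive the HUD and pause menu, and toggle a spawned grapple target indicator.
; Damage triggers camera shake, a delayed health-bar flash and a material parameter collection blink, while dynamic materials recolour hair and brows by health.
; A per-tick downward trace places a ground decal, scaled and faded by height.
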(event Custom|BlinkingMaterial
  ;[1 1 1] Take Damage Impl - Blink Material & Flash Health Widget
  (bind _value (Timeline|Blink PlayFromStart)
    (:Update
      (Rendering|Material|SetScalarParameterValue (Variables|Default|GetMP_PlayerDamage) (Utilities|Name|MakeLiteralName "BlinkValue") _value :!class /Script/Engine.KismetMaterialLibrary)
      (Rendering|Material|SetScalarParameterValue (Variables|Default|GetMP_PlayerDamage) (Utilities|Name|MakeLiteralName "BaseEmissive") (|(max((((2*x)-1)*m),0)) _value 0.3) :!class /Script/Engine.KismetMaterialLibrary))
    (:Finished
      (Rendering|Material|SetScalarParameterValue (Variables|Default|GetMP_PlayerDamage) (Utilities|Name|MakeLiteralName "BlinkValue") 1.0 :!class /Script/Engine.KismetMaterialLibrary)
      (Rendering|Material|SetScalarParameterValue (Variables|Default|GetMP_PlayerDamage) (Utilities|Name|MakeLiteralName "BaseEmissive") 0.0 :!class /Script/Engine.KismetMaterialLibrary))))

(event EventCancelAnimation
  ;[1 0.349 0.8177] Anim Activation Events
  ;;[1 1 1] Cancel
  (Animation|StopAnimMontage 0))

(event Collision|EventActorBeginOverlap
  (params (OtherActor :type Actor%20Object%20Reference)))

(event EventAttackSmackStart
  ;[1 0.9651 0.2083 1 37] Attack
  ;;[0.6806 0.5003 0.8281 1 20] Smack Attack
  (Animation|Montage|PlayMontage (Variables|Character|GetMesh) "/Game/Models/Pottitt/Animations/AnimMontages/AM_Smack_Potitt.AM_Smack_Potitt"
    (:OnBlendOut
      (Class|SteikemannCharacter|StopAttack))))

(event EventAnimonWallContact
  ;[1 0.349 0.8177] Anim Activation Events
  ;;[1 1 1] OnWall
  (Animation|Montage|PlayMontage (Variables|Character|GetMesh) "/Game/Models/Pottitt/Animations/AnimMontages/AM_OnWall_Contact_Potitt.AM_OnWall_Contact_Potitt"))

(event EventAnimPogoActive
  ;[1 0.349 0.8177] Anim Activation Events
  ;;[1 1 1] Pogo
  (Animation|Montage|PlayMontage (Variables|Character|GetMesh) "/Game/Models/Pottitt/Animations/AnimMontages/AM_Pogo_Active_Potitt.AM_Pogo_Active_Potitt"))

(event EventAnimTakeDamage
  ;[1 0.349 0.8177] Anim Activation Events
  ;;[1 1 1] Take Damage
  (Animation|Montage|PlayMontage (Variables|Character|GetMesh) "/Game/Models/Pottitt/Animations/AnimMontages/AM_TakeDamage_Potitt.AM_TakeDamage_Potitt"))

(event EventAnimGrappleStart
  ;[1 0.349 0.8177] Anim Activation Events
  ;;[1 1 1] Grapplehook
  (Animation|Montage|PlayMontage (Variables|Character|GetMesh) "/Game/Models/Pottitt/Animations/AnimMontages/AM_Grapple_Start_Potitt.AM_Grapple_Start_Potitt" 0.5))

(event EventAnimGrappleEnd
  ;[1 0.349 0.8177] Anim Activation Events
  ;;[1 1 1] Grapplehook
  (Animation|Montage|PlayMontage (Variables|Character|GetMesh) "/Game/Models/Pottitt/Animations/AnimMontages/AM_Grapple_End_Potitt.AM_Grapple_End_Potitt"))

(event EventAnimDeath
  ;[1 0.349 0.8177] Anim Activation Events
  ;;[1 1 1] Death
  (Animation|Montage|PlayMontage (Variables|Character|GetMesh) "/Game/Models/Pottitt/Animations/AnimMontages/AM_Death_Potitt.AM_Death_Potitt"))

(event EventAnimPogoPassive
  ;[1 0.349 0.8177] Anim Activation Events
  ;;[1 1 1] Pogo
  (Animation|Montage|PlayMontage (Variables|Character|GetMesh) "/Game/Models/Pottitt/Animations/AnimMontages/AM_Pogo_Passive_Potitt.AM_Pogo_Passive_Potitt"))

(event EventHealthHairColor
  (params (hp :type Integer))
  ;[1 1 1] Hair Color Change
  (CallFunction|HealthChangeMaterialUpdate hp))

(event EventTakeDamageImpl
  ;[1 1 1] Take Damage Impl - Blink Material & Flash Health Widget
  (CallFunction|TakeDamageWidgetUpdate)
  (CallFunction|BlinkingMaterial)
  (CameraShakes|StartCameraShake (Game|GetPlayerCameraManager 0) "/Game/Blueprints/Potitt/Camera/BP_DamageCameraShake.BP_DamageCameraShake_C" 1.0 "CameraLocal" "0, 0, 0"))

(event EventTick
  (params (DeltaSeconds :type Float%20%28single-precision%29))
  ;[0.9117 1 0.3133 1 39] Tick
  (CallFunction|GroundDecalPlacement))

(event EventAnimGroundPoundInitial
  ;[1 0.349 0.8177] Anim Activation Events
  ;;[1 1 1] Groundpound
  (Animation|Montage|PlayMontage (Variables|Character|GetMesh) "/Game/Models/Pottitt/Animations/Groundpound/AM_Groundpound_Initial_Potitt.AM_Groundpound_Initial_Potitt" (/ 1.0 (/ (Variables|Default|GetGP_PrePoundAirtime) (/ 5.0 3e+01)))))

(event EventAnimGroundPoundLandGround
  ;[1 0.349 0.8177] Anim Activation Events
  ;;[1 1 1] Groundpound
  (Animation|Montage|PlayMontage (Variables|Character|GetMesh) "/Game/Models/Pottitt/Animations/Groundpound/AM_Groundpound_Land_Potitt.AM_Groundpound_Land_Potitt"))

(event EventAnimLand
  (bind _returnvalue (Transformation|GetVelocity))
  ;[1 0.349 0.8177] Anim Activation Events
  ;;[1 0.2115 0.2115] Anim Land
  (if (and (and (> (Math|Vector|VectorLength (* _returnvalue "1.000000,1.000000,0.000000")) 1e+02) (< (.Z (Math|Vector|BreakVector _returnvalue)) -1.5e+03)) (> (Math|Vector|VectorLengthSquared (Variables|Default|Getm_InputVector)) 0.1))
    (Animation|Montage|PlayMontage (Variables|Character|GetMesh) "/Game/Models/Pottitt/Animations/AnimMontages/AM_Roll_Potitt.AM_Roll_Potitt")))

(event EventOnLanded
  (params (Hit :type Hit%20Result%20Structure%20%28by%20ref%29))
  ;[0.4737 0.4727 0.6302] Event Landed
  (Class|SteikemannCharacter|NSLandImplementation Hit)
  (Class|SteikemannCharacter|ResetState))

(event EventAnimActivateJump
  ;[1 0.349 0.8177] Anim Activation Events
  ;;[1 1 1] Jumps
  (Animation|Montage|PlayMontage (Variables|Character|GetMesh) "/Game/Models/Pottitt/Animations/AnimMontages/AM_Jump_Potitt.AM_Jump_Potitt"))

(event EventBeginPlay
  (bind _ground_decal (Variables|Default|GetGround-Decal))
  ;[1 0.3303 0.2904 1 39] Beginplay
  (Utilities|FlowControl|Sequence
    (:then_0
      (bind _returnvalue (Rendering|Material|CreateDynamicMaterialInstance (Class|DecalComponent|GetDecalMaterial _ground_decal) "None" "Transient" :!class /Script/Engine.KismetMaterialLibrary))
      (bind _output_get (Variables|Default|SetDynamicMat_GroundDecal _returnvalue))
      (Rendering|Components|Decal|SetDecalMaterial _ground_decal _output_get)
      (bind _returnvalue_2 (UserInterface|CreateWidget "/Game/Widget/WGT_HUD.WGT_HUD_C" (Game|GetPlayerController 0)))
      (bind _output_get_2 (Variables|Widgets|SetWGT%20HUD _returnvalue_2))
      (UserInterface|Viewport|AddtoViewport _returnvalue_2 0)
      (bind _returnvalue_3 (UserInterface|CreateWidget "/Game/Widget/PauseMenu/WGT_PauseMenu.WGT_PauseMenu_C" (Game|GetPlayerController 0)))
      (Variables|Widgets|SetWGT%20Pause%20Menu _returnvalue_3))
    (:then_1
      (CallFunction|CreateGrappleTargetIndicator)
      (CallFunction|UpdateAllCollectibles)
      (CallFunction|CreateDynamicHairMaterial))))

(event EventComboAttack
  (params (combo :type Integer))
  ;[1 0.9651 0.2083 1 37] Attack
  ;;[0.6806 0.5003 0.8281 1 20] Smack Attack
  (switch int combo
    (:1
      (Animation|Montage|PlayMontage (Variables|Character|GetMesh) "/Game/Models/Pottitt/Animations/AnimMontages/AM_Smack_Potitt.AM_Smack_Potitt"
        (:OnBlendOut
          _)))
    (:2
      (Animation|Montage|PlayMontage (Variables|Character|GetMesh) "/Game/Models/Pottitt/Animations/AnimMontages/AM_2ndSmack_Potitt.AM_2ndSmack_Potitt"
        (:OnBlendOut
          _))))
  (Class|SteikemannCharacter|StopAttack))

(event EventAnimActivateDoubleJump
  ;[1 0.349 0.8177] Anim Activation Events
  ;;[1 1 1] Jumps
  (Animation|Montage|PlayMontage (Variables|Character|GetMesh) "/Game/Models/Pottitt/Animations/AnimMontages/AM_DoubleJump_Potitt.AM_DoubleJump_Potitt"))

(event Custom|UpdateAllCollectibles
  ;[1 1 1] Update WGT_CollectibleCounter
)

(event Custom|Empty%20Ink%20Bottle
  ;[1 1 1] Ink Collectible
  (bind _inkbottle (Timeline|Empty%20Ink%20Bottle%20Timeline PlayFromStart)
    (:Update
      (Default|UpdateInkBottleValue (Variables|Widgets|GetWGT%20HUD) _inkbottle))))

(event Custom|Start_HealthFlashSubtraction
  ;[1 1 1] Health
  (bind _value (Timeline|HealthFlash PlayFromStart)
    (:Update
      (Default|UpdateHealthFlash (Variables|Widgets|GetWGT%20HUD) _value))
    (:Finished
      (Default|HealthFlashEnd (Variables|Widgets|GetWGT%20HUD)))))

(event Custom|TakeDamage_WidgetUpdate
  ;[1 1 1] Health
  (Default|HealthFlashStart (Variables|Widgets|GetWGT%20HUD))
  (bind _returnvalue (Utilities|Time|SetTimerbyEvent (delegate Custom|Start_HealthFlashSubtraction) 0.5))
  (Variables|Default|SetTH_StartHealthFlash _returnvalue))

(event EventUpdateInkCollectible
  ;[1 1 1] Ink Collectible
  (bind _addone (Timeline|Timeline PlayFromStart)
    (:Update
      (Default|UpdateInkBottleValue (Variables|Widgets|GetWGT%20HUD) (+ (/ (Math|Conversions|ToFloat(Integer) (- (Variables|Default|GetInkFlowerCollectible) 1)) 3.0) (/ _addone 3.0))))
    (:Finished
      (Class|SteikemannCharacter|CheckforNewJournalEntry))))

(event EventUpdateSapCollectible
  ;[1 1 1] Sap Collectible
  (Default|UpdateSap (Variables|Widgets|GetWGT%20HUD) (Variables|Default|GetCollectibleCommon)))

(event EventUpdateHealthWidget
  ;[1 1 1] Health
  (Default|UpdateHealth (Variables|Widgets|GetWGT%20HUD) (Variables|Default|GetHealth)))

(event EventShowHUDTimed
  ;[1 1 1] Update WGT_CollectibleCounter
  (Default|ShowInkBottle (Variables|Widgets|GetWGT%20HUD))
  (Class|SteikemannCharacter|UpdateSapCollectible)
  (Class|SteikemannCharacter|UpdateHealthWidget))

(event EventGetJournalEntry
  ;[1 1 1] Ink Collectible
  (Math|Integer|IncrementInt (Variables|Default|GetJournalEntries)
    (:%20%20
      (Utilities|Time|SetTimerbyEvent (delegate Custom|Empty%20Ink%20Bottle) 0.4)
      (Default|UnlockJournalEntry (Variables|Widgets|GetWGT%20HUD)))))

(event EventGainHealthImpl
  ;[1 1 1] Health
  (Utilities|Time|ClearandInvalidateTimerbyHandle (Variables|Default|GetTH_StartHealthFlash))
  (bind _value (Timeline|HealthFlash Stop)
    (:Update
      (Default|UpdateHealthFlash (Variables|Widgets|GetWGT%20HUD) _value))
    (:Finished
      (Default|HealthFlashEnd (Variables|Widgets|GetWGT%20HUD)))))

(event EventGHGrappleDynamicStart
  ;[1 1 1] Grapple Aim Indicator
  (Default|SetVisible (Variables|Default|GetBP%20Grapple%20Target%20Indicator) true))

(event EventGHGrappleDynamicEnd
  ;[1 1 1] Grapple Aim Indicator
  (Default|SetVisible (Variables|Default|GetBP%20Grapple%20Target%20Indicator) false))

(event EventGHAimIndicatorLocationDirection
  (params (Location :type Vector :default "0, 0, 0") (Normal :type Vector :default "0, 0, 0") (Direction :type Vector :default "0, 0, 0") (CameraDirection :type Vector :default "0, 0, 0"))
  ;[1 1 1] Grapple Aim Indicator
  (Default|SetTargetTransform (Variables|Default|GetBP%20Grapple%20Target%20Indicator) Location Normal Direction CameraDirection (Transformation|GetActorLocation)))

(event EventNewspaper
  ;[1 1 1] Ink Collectible
  (Default|NewspaperPickup (Variables|Widgets|GetWGT%20HUD))
  (Default|NewspaperPickup (Variables|Widgets|GetWGT%20Pause%20Menu)))

(event Input|ActionEvents|InputActionPauseMenu
  (params (Key :type Key%20Structure :default "None"))
  (bind _returnvalue (Game|GetPlayerController 0))
  (bind _wgt_pause_menu (Variables|Widgets|GetWGT%20Pause%20Menu))
  (bind _wgt_pause_menu_2 (Variables|Widgets|GetWGT%20Pause%20Menu))
  ;[1 0.5936 0.6036 1 40] Pause Menu
  (:Pressed
    (if (Game|IsGamePaused)
      ;;[1 1 1] Close
      (Game|SetGamePaused false)
      (Default|RemoveControlsWidgets _wgt_pause_menu_2)
      (Widget|RemovefromParent _wgt_pause_menu_2)
      (Input|SetInputModeGameOnly _returnvalue false)
      (Variables|/Script/Engine.PlayerController|SetbEnableClickEvents _returnvalue false)
      (Variables|/Script/Engine.PlayerController|SetbShowMouseCursor _returnvalue false)
      (else
        ;;[0.2219 0.2219 0.2219] Open
        (Game|SetGamePaused true)
        (Variables|/Script/Engine.PlayerController|SetbShowMouseCursor (Game|GetPlayerController 0) true)
        (UserInterface|Viewport|AddtoViewport (Variables|Widgets|GetWGT%20Pause%20Menu) 0)
        (bind _output_get (Variables|Default|SetGamePad%20Menu%20Button 0))
        (Default|SetButtonHovered _wgt_pause_menu _output_get)
        (Default|WidgetEnter _wgt_pause_menu (Variables|Default|GetCollectedNewspapers_WidgetIndexes))
        (Default|GetCollectibleInfo _wgt_pause_menu (Variables|Default|GetCollectibleCommon) (Variables|Default|GetHealth) (Variables|Default|GetInkFlowerCollectible) (Variables|Default|GetJournalEntries))
        (Input|SetInputModeGameandUI (Game|GetPlayerController 0) (Variables|Widgets|GetWGT%20Pause%20Menu) "DoNotLock" true false)))))

(event Input|ActionEvents|InputActionMenu_Interact_MnK
  (params (Key :type Key%20Structure :default "None"))
  ;[0.3177 0.3177 0.3177 1 40] Gamepad / Keyboard Menu Interaction
  ;;[0.5312 0.5312 0.5312 1 25] On Menu Interaction
)

(event Input|ActionEvents|InputActionMenu_Interact_Gamepad
  (params (Key :type Key%20Structure :default "None"))
  ;[0.3177 0.3177 0.3177 1 40] Gamepad / Keyboard Menu Interaction
  ;;[0.5312 0.5312 0.5312 1 25] On Menu Interaction
)

(event Input|AxisEvents|InputAxisMenuNavigation_Y
  (params (AxisValue :type Float%20%28single-precision%29))
  ;[0.3177 0.3177 0.3177 1 40] Gamepad / Keyboard Menu Interaction
)

(fn ConstructionScript)

(fn GroundDecalPlacement
  (bind _zlength (LocalVariables|GetZLength))
  (bind (_outhit _returnvalue) (Collision|LineTraceByChannel (Transformation|GetActorLocation) (- (Transformation|GetActorLocation) (Math|Vector|MakeVector 0.0 0.0 (LocalVariables|GetRayLength))) "TraceTypeQuery1" false 0 "None"))
  (if _returnvalue
    ;[1 1 1] Set decal to location beneath character
    (Transformation|SetWorldLocation (Variables|Default|GetGround-Decal) (.ImpactPoint (Collision|BreakHitResult _outhit)) false false)
    ;[1 1 1] Decal scale based on length to ground based on max ZLength
    (Rendering|Material|SetScalarParameterValue (Variables|Default|GetDynamicMat_GroundDecal) "Density" (Math|Curves|GetFloatValue (Variables|Default|GetCurve_DecalAlpha) (/ (Math|Float|Clamp(Float) (Math|Vector|VectorLength (- (.ImpactPoint (Collision|BreakHitResult _outhit)) (Transformation|GetActorLocation))) 0.0 _zlength) _zlength)) :!class /Script/Engine.MaterialInstanceDynamic)
    (Transformation|SetWorldScale3D (Variables|Default|GetGround-Decal) (Math|Vector|MakeVector (* (Math|Curves|GetFloatValue (Variables|Default|GetCurve_DecalAlpha) (/ (Math|Float|Clamp(Float) (Math|Vector|VectorLength (- (.ImpactPoint (Collision|BreakHitResult _outhit)) (Transformation|GetActorLocation))) 0.0 _zlength) _zlength)) 5.0) 1.0 1.0))))

(fn CreateDynamicHairMaterial
  (bind _browmaterialindex (LocalVariables|GetBrowMaterialIndex))
  (bind _hairmaterialindex (LocalVariables|GetHairMaterialIndex))
  ;[0 0 0] Hair
  (bind _returnvalue (Rendering|Material|CreateDynamicMaterialInstance (Rendering|Material|GetMaterial (Variables|Character|GetMesh) _hairmaterialindex) "HairMat" "Transient" :!class /Script/Engine.KismetMaterialLibrary))
  (bind _output_get (Variables|HairMaterial|SetHair_DynamicMaterial _returnvalue))
  (Rendering|Material|SetMaterial (Variables|Character|GetMesh) _hairmaterialindex _output_get)
  ;[0 0 0] Brow
  (bind _returnvalue_2 (Rendering|Material|CreateDynamicMaterialInstance (Rendering|Material|GetMaterial (Variables|Character|GetMesh) _browmaterialindex) "BrowMat" "Transient" :!class /Script/Engine.KismetMaterialLibrary))
  (bind _output_get_2 (Variables|HairMaterial|SetBrow_DynamicMaterial _returnvalue_2))
  (Rendering|Material|SetMaterial (Variables|Character|GetMesh) _browmaterialindex _output_get_2))

(fn CreateGrappleTargetIndicator
  (bind _returnvalue (Game|SpawnActorfromClass "/Game/Blueprints/Potitt/BP_GrappleTargetIndicator.BP_GrappleTargetIndicator_C" (Math|Transform|MakeTransform (Transformation|GetActorLocation)) "Undefined" 0 0))
  (bind _output_get (Variables|Default|SetBP%20Grapple%20Target%20Indicator _returnvalue))
  (Default|SetVisible _output_get false))

(fn HealthChangeMaterialUpdate
  (params (Health :type Integer))
  (bind _parametername (LocalVariables|GetParameterName))
  (bind _parametername_2 (LocalVariables|GetParameterName))
  (switch int Health
    (:1
      (Rendering|Material|SetTextureParameterValue (Variables|HairMaterial|GetHair_DynamicMaterial) _parametername_2 "/Game/Textures/Pottit_tex/Hair_brown_BaseColor.Hair_brown_BaseColor")
      (Rendering|Material|SetTextureParameterValue (Variables|HairMaterial|GetBrow_DynamicMaterial) _parametername "/Game/Textures/Pottit_tex/Brow_brown_BaseColor.Brow_brown_BaseColor"))
    (:2
      (Rendering|Material|SetTextureParameterValue (Variables|HairMaterial|GetHair_DynamicMaterial) _parametername_2 "/Game/Textures/Pottit_tex/Hair_red_BaseColor.Hair_red_BaseColor")
      (Rendering|Material|SetTextureParameterValue (Variables|HairMaterial|GetBrow_DynamicMaterial) _parametername "/Game/Textures/Pottit_tex/Brow_red_BaseColor.Brow_red_BaseColor"))
    (:3
      (Rendering|Material|SetTextureParameterValue (Variables|HairMaterial|GetHair_DynamicMaterial) _parametername_2 "/Game/Textures/Pottit_tex/hair_yellow_BaseColor.hair_yellow_BaseColor")
      (Rendering|Material|SetTextureParameterValue (Variables|HairMaterial|GetBrow_DynamicMaterial) _parametername "/Game/Textures/Pottit_tex/brow_yellow_BaseColor.brow_yellow_BaseColor"))
    (:4
      (Rendering|Material|SetTextureParameterValue (Variables|HairMaterial|GetHair_DynamicMaterial) _parametername_2 "/Game/Textures/Pottit_tex/hair_green_BaseColor.hair_green_BaseColor")
      (Rendering|Material|SetTextureParameterValue (Variables|HairMaterial|GetBrow_DynamicMaterial) _parametername "/Game/Textures/Pottit_tex/brow_green_BaseColor.brow_green_BaseColor"))))