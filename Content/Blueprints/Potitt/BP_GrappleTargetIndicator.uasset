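; BP_GrappleTargetIndicator is an actor with sphere and plane meshes that serves as a grapple target marker.
; BeginPlay gives both meshes dynamic material instances and stores them in DynamicMaterials.
; SetVisible toggles the whole component tree from the root, while SetTargetTransform only moves the actor to the given location.
; Camera-facing plane rotation and distance-scaled emissive strength are present but disconnected, so they never run.
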(event `self.ReceiveBeginPlay`
  (bind _sphere (`self.Sphere`))
  (bind _plane (`self.Plane`))
  ;[0.3385 0.3385 0.3385] Creating and setting dynamic material
  (bind _returnvalue (`PrimitiveComponent.CreateDynamicMaterialInstance` _sphere 0 (`PrimitiveComponent.GetMaterial` _sphere 0) "None"))
  (`KismetArrayLibrary.Array_Add` (`self.DynamicMaterials`) _returnvalue)
  (bind _returnvalue_2 (`PrimitiveComponent.CreateDynamicMaterialInstance` _plane 0 (`PrimitiveComponent.GetMaterial` _plane 0) "None"))
  (`KismetArrayLibrary.Array_Add` (`self.DynamicMaterials`) _returnvalue_2)
  (`PrimitiveComponent.SetMaterial` (`self.Sphere`) 0 (`|GetArrayItem` (`self.DynamicMaterials`)))
  (`PrimitiveComponent.SetMaterial` (`self.Plane`) 0 (`|GetArrayItem` (`self.DynamicMaterials`) 1)))

(event `self.ReceiveTick`
  (params (DeltaSeconds :type "Float (single-precision)")))

(fn `SetTargetTransform`
  (params (Location :type "Vector Structure") (Normal :type "Vector Structure") (Direction :type "Vector Structure") (CameraDirection :type "Vector Structure") (PlayerLocation :type "Vector Structure"))
  (locals (DivideLengthForEmissive :type "Float (double-precision)" :default 400.0))
  (`|ExecutionSequence`
    (:`then_0`
      (`self.K2_SetActorLocation` (`local.Location`)))))

(fn `SetVisible`
  (params (Visible :type Boolean))
  (`SceneComponent.SetVisibility` (`self.DefaultSceneRoot`) Visible true))

(fn `UserConstructionScript`)