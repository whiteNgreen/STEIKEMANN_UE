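; Player character Blueprint for TheSteikemann, handling jump, dash and attack montages, landing, and the pause menu.
; Attacks share an anticipation montage, then DecideAttackType branches to Smack or Scoop, with chained blend-outs toggling the attack collider.
; The pause menu takes gamepad or keyboard axis navigation with wrap-around selection.
; Debug features include an optional aim-marker widget, camera-shake keys, ground-pound collider display, and a G-held vertical velocity test run on Tick.
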(event `self.ReceiveBeginPlay`
  ;[1 0.3303 0.2904 1 39] Beginplay
  (if (`self.bShowAimingLocaiton_Debug`)
    (bind _returnvalue (`|CreateWidget` "/Game/Widget/WGT_AimMarker.WGT_AimMarker_C" (`GameplayStatics.GetPlayerController` 0)))
    (bind _output_get (set `self.AimMarkerWidget` _returnvalue))
    (`UserWidget.AddToViewport` _output_get 0)))

(event `self.ReceiveTick`
  (params (DeltaSeconds :type "Float (single-precision)"))
  (`self.Velocity Test`))

(event `InputAction|Dash`
  (params (Key :type "Key Structure")))

(event `Key|T`
  (params (Key :type "Key Structure"))
  (:`Pressed`
    (`GameplayStatics.PlayWorldCameraShake` "/Game/Blueprints/Potitt/Camera/BP_CameraShake1.BP_CameraShake1_C" (+ (`SceneComponent.K2_GetComponentLocation` (`self.Camera`)) (0.0 0.0 1.0)) 0.0 10.0 50.0)))

(event `self.Anim_Activate_Jump`
  (`|PlayMontage` (`self.Mesh`) "/Game/Models/Cube/Animations/AM_Jump-Start.AM_Jump-Start"))

(event `Key|Y`
  (params (Key :type "Key Structure"))
  (:`Pressed`
    (`GameplayStatics.PlayWorldCameraShake` "/Game/Blueprints/Potitt/Camera/CS_Pitch-Shake.CS_Pitch-Shake_C" (`self.K2_GetActorLocation`) 0.0 10.0 0.0 true)))

(event `Key|U`
  (params (Key :type "Key Structure"))
  (:`Pressed`
    (`GameplayStatics.PlayWorldCameraShake` "/Game/Blueprints/Potitt/Camera/CS_Jump_Land.CS_Jump_Land_C" (+ (`SceneComponent.K2_GetComponentLocation` (`self.Camera`)) (0.0 0.0 1.0)) 0.0 10.0 50.0)))

(event `self.Activate_Dash`
  (`|PlayMontage` (`self.Mesh`) "/Game/Models/Cube/Animations/AM_Pre-Dash.AM_Pre-Dash"
    (:`OnCompleted`
      (`|PlayMontage` (`self.Mesh`) "/Game/Models/Cube/Animations/AM_Dash.AM_Dash"))))

(event `Key|AnyKey`
  (params (Key :type "Key Structure"))
  ;[1 1 1] Testing for raw input og ps4 kontroller
)

(event `Key|T`
  (params (Key :type "Key Structure"))
  (bind _groundpoundcollider (`self.GroundPoundCollider`))
  (:`Pressed`
    (`SphereComponent.SetSphereRadius` _groundpoundcollider 300.0 true)
    (if (`SceneComponent.bHiddenInGame` _groundpoundcollider)
      (`SceneComponent.SetHiddenInGame` (`self.GroundPoundCollider`) false false)
      (else
        (`SceneComponent.SetHiddenInGame` (`self.GroundPoundCollider`) true false)))))

(event `InputAction|PauseMenu` :paused true
  (params (Key :type "Key Structure"))
  (bind _wgt_pause_menu (`self.WGT Pause Menu`))
  ;[0.7756 1 0.9185 1 85] UI
  ;;[1 0.5936 0.6036 1 40] Pause Menu
  (:`Pressed`
    (if (`GameplayStatics.IsGamePaused`)
      (`GameplayStatics.SetGamePaused` false)
      (`Widget.RemoveFromParent` (`self.WGT Pause Menu`))
      (else
        (`GameplayStatics.SetGamePaused` true)
        (set `PlayerController.bShowMouseCursor` true (`GameplayStatics.GetPlayerController` 0))
        (bind _returnvalue (`|CreateWidget` "/Game/Widget/WGT_PauseMenu.WGT_PauseMenu_C" (`GameplayStatics.GetPlayerController` 0)))
        (bind _output_get (set `self.WGT Pause Menu` _returnvalue))
        (`UserWidget.AddToViewport` _output_get 0)
        (bind _output_get_2 (set `self.GamePad Menu Button` 0))
        (`/Game/Widget/WGT_PauseMenu.SetButtonHovered` _wgt_pause_menu _output_get_2)
        (`WidgetBlueprintLibrary.SetInputMode_GameAndUIEx` (`GameplayStatics.GetPlayerController` 0) _wgt_pause_menu)))))

(event `self.OnLanded`
  (params (Hit :type "HitResult Structure (by ref)"))
  ;[0.4737 0.4727 0.6302] Event Landed
  (`self.NS_Land_Implementation` Hit))

(event `InputAxis|MenuNavigation_Y` :paused true
  (params (AxisValue :type "Float (single-precision)"))
  (bind _returnvalue (`KismetMathLibrary.Round` (* AxisValue -1.0)))
  ;[0.7756 1 0.9185 1 85] UI
  ;;[0 0 0 1 40] Gamepad / Keyboard Menu Interaction
  (if (`GameplayStatics.IsGamePaused`)
    (if (== _returnvalue 0)
      (goto _label :!via `Reset`)
      (else
        (`/Engine/EditorBlueprintResources/StandardMacros.DoOnce` false :!label _label
          (:`Completed`
            (set `self.GamePad Menu Button` (+ (`self.GamePad Menu Button`) _returnvalue))
            (`|ExecutionSequence`
              (:`then_0`
                (if (< (`self.GamePad Menu Button`) 0)
                  (set `self.GamePad Menu Button` (- (`KismetArrayLibrary.Array_Length` (`/Game/Widget/WGT_PauseMenu.Buttons` (`self.WGT Pause Menu`))) 1))))
              (:`then_1`
                (if (> (`self.GamePad Menu Button`) (- (`KismetArrayLibrary.Array_Length` (`/Game/Widget/WGT_PauseMenu.Buttons` (`self.WGT Pause Menu`))) 1))
                  (set `self.GamePad Menu Button` 0)))
              (:`then_2`
                (`/Game/Widget/WGT_PauseMenu.SetButtonHovered` (`self.WGT Pause Menu`) (`self.GamePad Menu Button`))))))))))

(event `InputAction|Menu_Interact` :paused true
  (params (Key :type "Key Structure"))
  ;[0.7756 1 0.9185 1 85] UI
  ;;[0 0 0 1 40] Gamepad / Keyboard Menu Interaction
  ;;;[0.5312 0.5312 0.5312 1 25] On Menu Interaction
  (:`Pressed`
    (if (`GameplayStatics.IsGamePaused`)
      (`/Game/Widget/WGT_PauseMenu.ClickButton` (`self.WGT Pause Menu`) (`self.GamePad Menu Button`)))))

(event `Key|G`
  (params (Key :type "Key Structure"))
  ;[1 1 1] Attacks Smack & Scoop testing
  (:`Pressed`
    (set `self.bGpressed` true))
  (:`Released`
    (set `self.bGpressed` false)))

(event `self.Start_Attack`
  ;[1 0.9651 0.2083 1 37] Attack
  (`self.Start_Attack_Pure`)
  ;;[1 1 1] Starting with the same anticipation
  (`|PlayMontage` (`self.Mesh`) "/Game/Models/AdvancedCubeRig/Animations/Montages/SmackAttack/AM_SmackAttack_Anticipation.AM_SmackAttack_Anticipation" (`self.BasicAttack_CommonAnticipation_Rate`)
    (:`OnBlendOut`
      ;;[1 1 1] If button is still held do scoop, else do smack
      (if (`self.DecideAttackType`)
        ;;[0.5678 0.7708 0.554] Scoop Attack
        (`|PlayMontage` (`self.Mesh`) "/Game/Models/AdvancedCubeRig/Animations/Montages/ScoopAttack/AM_ScoopAttack_Anticipation.AM_ScoopAttack_Anticipation" (`self.ScoopAttack_Anticipation_Rate`)
          (:`OnBlendOut`
            (`self.Activate_AttackCollider`)
            (`|PlayMontage` (`self.Mesh`) "/Game/Models/AdvancedCubeRig/Animations/Montages/ScoopAttack/AM_ScoopAttack_Action.AM_ScoopAttack_Action" (`self.ScoopAttack_Action_Rate`)
              (:`OnBlendOut`
                (`self.Deactivate_ScoopAttack`)
                (`self.Deactivate_AttackCollider`)
                (`|PlayMontage` (`self.Mesh`) "/Game/Models/AdvancedCubeRig/Animations/Montages/ScoopAttack/AM_ScoopAttack_Reaction.AM_ScoopAttack_Reaction" (`self.ScoopAttack_Reaction_Rate`)
                  (:`OnBlendOut`
                    (`self.Stop_Attack`)))))))
        (else
          ;;[0.6806 0.5003 0.8281 1 20] Smack Attack
          (`self.Activate_AttackCollider`)
          (`|PlayMontage` (`self.Mesh`) "/Game/Models/AdvancedCubeRig/Animations/Montages/SmackAttack/AM_SmackAttack_Action.AM_SmackAttack_Action" (`self.SmackAttack_Action_Rate`)
            (:`OnBlendOut`
              (`self.Deactivate_SmackAttack`)
              (`self.Deactivate_AttackCollider`)
              (`|PlayMontage` (`self.Mesh`) "/Game/Models/AdvancedCubeRig/Animations/Montages/SmackAttack/AM_SmackAttack_Reaction.AM_SmackAttack_Reaction" (`self.SmackAttack_Reaction_Rate`)
                (:`OnBlendOut`
                  (`self.Stop_Attack`))))))))))

(fn `ForceTest`
  (bind _charactermovement (`self.CharacterMovement`))
  (if (`self.bGpressed`)
    ;[1 1 1] Kan bruke denne for å stå rellativt stille i lufta.
    ; Kan hende spilleren flyter litt opp over forlenget bruk, men den skal aldri brukes så lenge
    (`CharacterMovementComponent.AddForce` _charactermovement (`KismetMathLibrary.MakeVector` 0.0 0.0 (* (* (`MovementComponent.GetGravityZ` _charactermovement) -1.0) (`CharacterMovementComponent.Mass` _charactermovement))))))

(fn `NewFunction_0`
  (params (NewParam :type Boolean))
  (returns (NewParam1 :type Boolean))
  (return false))

(fn `UserConstructionScript`)

(fn `Velocity Test`
  (locals (NewLocalVar_0 :type "Float (double-precision)" :default 100.0))
  (bind _charactermovement (`self.CharacterMovement`))
  (if (`self.bGpressed`)
    ;[1 1 1] Timer
    (set `self.Timer` (+ (`self.Timer`) (`GameplayStatics.GetWorldDeltaSeconds`)))
    ;[1 1 1] Velocity
    (set `MovementComponent.Velocity` (`KismetMathLibrary.MakeVector` 0.0 0.0 (+ (* (* (`MovementComponent.GetGravityZ` (`self.CharacterMovement`)) -1.0) (`GameplayStatics.GetWorldDeltaSeconds`)) 100.0)) _charactermovement)
    (`CharacterMovementComponent.SetMovementMode` _charactermovement "MOVE_Falling" 0)
    ;[1 1 1] Printing Height
    (if (>= (`self.Timer`) 1.0)
      (`KismetSystemLibrary.PrintString` (`KismetStringLibrary.Concat_StrStr` "Height: " (`KismetStringLibrary.Conv_DoubleToString` (- (.z (`self.K2_GetActorLocation`)) (`CapsuleComponent.GetScaledCapsuleHalfHeight` (`self.CapsuleComponent`))))) true true (struct :`G` 0.333333 :`B` 0.132948 :`A` 1.0))
      (set `self.Timer` 0.0))
    (else
      (set `self.Timer` 0.0))))