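; Player controller that tracks the player's current input type and shares changes with the character and any listeners.
; Any key press is passed to CheckInputType for detection.
; ChangedInputType copies MEInputType to a valid PlayerCharacter, then calls the input type event dispatcher.
; The two movement axis events only reach an IsGamePaused branch with nothing after it.
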(event `self.ChangedInputType`
  (bind _playercharacter (`self.PlayerCharacter`))
  (`/Engine/EditorBlueprintResources/StandardMacros.IsValid` _playercharacter
    (:`Is Valid`
      (set `SteikemannCharacter.m_EInputType` (`self.m_EInputType`) _playercharacter))
    (:`Is Not Valid`
      _))
  (`self.InputTypeEventDispatcher` (`self.m_EInputType`)))

(event `Key|AnyKey` :consume false :paused true :overrideparent false
  (params (Key :type "Key Structure"))
  (:`Pressed`
    (`self.CheckInputType` Key)))

(event `InputAxis|Move Forward / Backward` :consume false :paused true
  (params (AxisValue :type "Float (single-precision)"))
  (if (`GameplayStatics.IsGamePaused`) :!label _label
    _))

(event `InputAxis|Move Right / Left` :consume false :paused true
  (params (AxisValue :type "Float (single-precision)"))
  (goto _label))

(fn `UserConstructionScript`)