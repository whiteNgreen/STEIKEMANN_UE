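; Main menu pawn that shows the menu widget and handles the transition from the "Press Any Button" screen to the main menu.
; On begin play it enables cursor and UI input and snaps its camera to ViewOne, with both view components deactivated as transform markers.
; Any key fades out the first screen, starts a timer for the menu fade-in and enables a Tick-driven, eased camera move to ViewTwo.
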(event `self.ReceiveBeginPlay`
  (bind _returnvalue (`GameplayStatics.GetPlayerController` 0))
  (set `PlayerController.bShowMouseCursor` true _returnvalue)
  (bind _returnvalue_2 (`|CreateWidget` "/Game/Widget/MainMenu/WGT_MainMenu.WGT_MainMenu_C" _returnvalue))
  (`UserWidget.AddToViewport` _returnvalue_2 0)
  (`WidgetBlueprintLibrary.SetInputMode_GameAndUIEx` _returnvalue _returnvalue_2)
  (set `self.MainMenu_Widget` _returnvalue_2)
  (`ActorComponent.Deactivate` (`self.View_One`))
  (`ActorComponent.Deactivate` (`self.View_Two`))
  (`SceneComponent.K2_SetWorldLocationAndRotation` (`self.Camera`) (.location (`SceneComponent.K2_GetComponentToWorld` (`self.View_One`))) (.rotation (`SceneComponent.K2_GetComponentToWorld` (`self.View_One`))) false false))

(event `self.ReceiveTick`
  (params (DeltaSeconds :type "Float (single-precision)"))
  (if (`self.bCameraLerp`)
    (`self.CameraLerp` DeltaSeconds)))

(event `Key|AnyKey`
  (params (Key :type "Key Structure"))
  (:`Pressed`
    (switch `/Game/Widget/MainMenu/MainMenuState` (`self.State`)
      (:`NewEnumerator0`
        (`/Game/Widget/MainMenu/WGT_MainMenu.First_FadeOut` (`self.MainMenu_Widget`))
        (set `self.State` "NewEnumerator2")
        (`KismetSystemLibrary.K2_SetTimerDelegate` (delegate `Start Main Menu Fade In`) 2.0)
        (set `self.bCameraLerp` true)))))

(event `Start Main Menu Fade In`
  (set `self.State` "NewEnumerator1")
  (`/Game/Widget/MainMenu/WGT_MainMenu.MainMenu_FadeIn` (`self.MainMenu_Widget`)))

(fn `CameraLerp`
  (params (DeltaTime :type "Float (double-precision)"))
  (returns (ReachedTarget :type Boolean))
  (set `self.CamLerpAlpha` (`KismetMathLibrary.FClamp` (+ (* DeltaTime (`self.CamLerpSpeed`)) (`self.CamLerpAlpha`))))
  (`SceneComponent.K2_SetWorldLocationAndRotation` (`self.Camera`) (`|EaseFunction` "EaseInOut" (`self.CamLerpAlpha`) (.location (`SceneComponent.K2_GetComponentToWorld` (`self.View_One`))) (.location (`SceneComponent.K2_GetComponentToWorld` (`self.View_Two`)))) (`|EaseFunction` "EaseInOut" (`self.CamLerpAlpha`) (.rotation (`SceneComponent.K2_GetComponentToWorld` (`self.View_One`))) (.rotation (`SceneComponent.K2_GetComponentToWorld` (`self.View_Two`)))) false false)
  (return false))

(fn `UserConstructionScript`)