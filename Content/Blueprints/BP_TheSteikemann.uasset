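; Player Blueprint for the Steikemann that handles the pause menu and early controller-detection logic.
; The pause input toggles game pause and WGT_PauseMenu; while paused, a rounded, DoOnce-gated axis moves a wrapping button highlight and the interact input clicks it.
; Controller detection cuts vendor and product IDs from registered device names, but its handler is a stub and the N key prints the IDs for debugging.
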(event `self.OnControllerConnection`
  (if (== (`KismetArrayLibrary.Array_Length` (`RawInputFunctionLibrary.GetRegisteredDevices`)) 0)
    (`self.GetControllerData`)))

(event `GetControllerData`
  (for _array_element (`RawInputFunctionLibrary.GetRegisteredDevices`)
    (bind (_handle _vendorid _productid _devicename) (break `RegisteredDeviceInfo` _array_element))
    (set `self.Current Controller VID` (`KismetStringLibrary.GetSubstring` _devicename 12 4))
    (set `self.Current Controller PID` (`KismetStringLibrary.GetSubstring` _devicename 21 4)))
  (`self.HandleConnectedController`))

(event `self.ReceiveBeginPlay`
  ;[1 0.3303 0.2904 1 39] Beginplay
)

(event `InputAction|Dash`
  (params (Key :type "Key Structure")))

(event `self.ReceiveTick`
  (params (DeltaSeconds :type "Float (single-precision)")))

(event `OnControllerDetected`
  (params (CurrentController :type Byte)))

(event `Key|AnyKey`
  (params (Key :type "Key Structure")))

(event `Key|N`
  (params (Key :type "Key Structure"))
  (:`Pressed`
    (`KismetSystemLibrary.PrintString` (`self.Current Controller VID`) true true (struct :`R` 1.0 :`B` 0.817722 :`A` 1.0))
    (`KismetSystemLibrary.PrintString` (`self.Current Controller PID`) true true (struct :`R` 1.0 :`G` 0.878595 :`A` 1.0))
    (for _array_element (`RawInputFunctionLibrary.GetRegisteredDevices`)
      (bind (_handle _vendorid _productid _devicename) (break `RegisteredDeviceInfo` _array_element))
      (`KismetSystemLibrary.PrintString` (`KismetStringLibrary.GetSubstring` _devicename 12 4) true true (struct :`G` 0.317708 :`B` 0.13017 :`A` 1.0))
      (`KismetSystemLibrary.PrintString` (`KismetStringLibrary.GetSubstring` _devicename 21 4) true true (struct :`G` 0.317708 :`B` 0.13017 :`A` 1.0)))))

(event `InputAction|PauseMenu` :paused true
  (params (Key :type "Key Structure"))
  (bind _wgt_pause_menu (`self.WGT Pause Menu`))
  ;[0.7756 1 0.9185 1 85] UI
  ;;[1 0.5936 0.6036 1 40] Pause Menu
  (:`Pressed`
    (if (`GameplayStatics.IsGamePaused`)
      (`GameplayStatics.SetGamePaused` false)
      (`Widget.RemoveFromParent` (`self.WGT Pause Menu`))
      (else
        (`GameplayStatics.SetGamePaused` true)
        (set `PlayerController.bShowMouseCursor` true (`GameplayStatics.GetPlayerController` 0))
        (bind _returnvalue (`|CreateWidget` "/Game/Widget/WGT_PauseMenu.WGT_PauseMenu_C" (`GameplayStatics.GetPlayerController` 0)))
        (bind _output_get (set `self.WGT Pause Menu` _returnvalue))
        (`UserWidget.AddToViewport` _output_get 0)
        (bind _output_get_2 (set `self.GamePad Menu Button` 0))
        (`/Game/Widget/WGT_PauseMenu.SetButtonHovered` _wgt_pause_menu _output_get_2)
        (`WidgetBlueprintLibrary.SetInputMode_GameAndUIEx` (`GameplayStatics.GetPlayerController` 0) _wgt_pause_menu)))))

(event `HandleConnectedController`
  (if (`KismetStringLibrary.EqualEqual_StrStr` (`self.Current Controller VID`) (`self.Current Controller PID`))
    _))

(event `InputAxis|MenuNavigation_Y` :paused true
  (params (AxisValue :type "Float (single-precision)"))
  (bind _returnvalue (`KismetMathLibrary.Round` (* AxisValue -1.0)))
  ;[0.7756 1 0.9185 1 85] UI
  ;;[0 0 0 1 40] Gamepad / Keyboard Menu Interaction
  (if (`GameplayStatics.IsGamePaused`)
    (if (== _returnvalue 0)
      (goto _label :!via `Reset`)
      (else
        (`/Engine/EditorBlueprintResources/StandardMacros.DoOnce` false :!label _label
          (:`Completed`
            (set `self.GamePad Menu Button` (+ (`self.GamePad Menu Button`) _returnvalue))
            (`|ExecutionSequence`
              (:`then_0`
                (if (< (`self.GamePad Menu Button`) 0)
                  (set `self.GamePad Menu Button` (- (`KismetArrayLibrary.Array_Length` (`/Game/Widget/WGT_PauseMenu.Buttons` (`self.WGT Pause Menu`))) 1))))
              (:`then_1`
                (if (> (`self.GamePad Menu Button`) (- (`KismetArrayLibrary.Array_Length` (`/Game/Widget/WGT_PauseMenu.Buttons` (`self.WGT Pause Menu`))) 1))
                  (set `self.GamePad Menu Button` 0)))
              (:`then_2`
                (`/Game/Widget/WGT_PauseMenu.SetButtonHovered` (`self.WGT Pause Menu`) (`self.GamePad Menu Button`))))))))))

(event `InputAction|Menu_Interact` :paused true
  (params (Key :type "Key Structure"))
  ;[0.7756 1 0.9185 1 85] UI
  ;;[0 0 0 1 40] Gamepad / Keyboard Menu Interaction
  ;;;[0.5312 0.5312 0.5312 1 25] On Menu Interaction
  (:`Pressed`
    (if (`GameplayStatics.IsGamePaused`)
      (`/Game/Widget/WGT_PauseMenu.ClickButton` (`self.WGT Pause Menu`) (`self.GamePad Menu Button`)))))

(fn `UserConstructionScript`)