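; Placeable trigger volume that loads or unloads a streaming level when the player enters its box.
; Overlaps only count for a capsule component on an actor carrying the Pottit gameplay tag.
; LoadOption selects a blocking load, made visible afterwards, or a blocking unload of the referenced level.
; The construction script labels the trigger with the level name and mode, colour-coded by load or unload.
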(event `self.ReceiveBeginPlay`)

(event `self.Box.OnComponentBeginOverlap`
  (params (OverlappedComponent :type "PrimitiveComponent Object Reference") (OtherActor :type "Actor Object Reference") (OtherComp :type "PrimitiveComponent Object Reference") (OtherBodyIndex :type Integer) (bFromSweep :type Boolean) (SweepResult :type "HitResult Structure (by ref)"))
  (bind _level (`self.Level`))
  (if (`self.Collides with Player` OtherActor OtherComp)
    (switch `/Game/Blueprints/LevelStreaming/StreamingOption` (`self.LoadOption`)
      (:`NewEnumerator0`
        (`GameplayStatics.LoadStreamLevelBySoftObjectPtr` _level true true))
      (:`NewEnumerator1`
        (`GameplayStatics.UnloadStreamLevelBySoftObjectPtr` _level true)))))

(fn `Collides with Player`
  (params (Actor :type "Actor Object Reference") (Comp :type "ActorComponent Object Reference"))
  (returns (ReturnValue :type Boolean))
  (if (== (`GameplayStatics.GetObjectClass` Comp) "/Script/Engine.CapsuleComponent")
    (bind _returnvalue (message `GameplayTagAssetInterface.HasMatchingGameplayTag` Actor (struct :`TagName` "Pottit")))
    (return _returnvalue)))

(fn `UserConstructionScript`
  (locals (LoadTypeText :type Text) (LoadColor :type "Color Structure" :default (struct :`B` 255 :`G` 43 :`R` 28 :`A` 255)) (UnloadColor :type "Color Structure" :default (struct :`G` 20 :`R` 255 :`A` 255)))
  (bind _unloadcolor (`local.UnloadColor`))
  (bind _loadcolor (`local.LoadColor`))
  (`TextRenderComponent.K2_SetText` (`self.TextRender`) (`KismetTextLibrary.Conv_NameToText` (`self.Level Name`)))
  (switch `/Game/Blueprints/LevelStreaming/StreamingOption` (`self.LoadOption`)
    (:`NewEnumerator0`
      (bind _output_get (set `local.LoadTypeText` "Load Level"))
      (`TextRenderComponent.K2_SetText` (`self.TextRender1`) _output_get)
      (`TextRenderComponent.SetTextRenderColor` (`self.TextRender`) _loadcolor)
      (`TextRenderComponent.SetTextRenderColor` (`self.TextRender1`) _loadcolor))
    (:`NewEnumerator1`
      (bind _output_get_2 (set `local.LoadTypeText` "Unload Level"))
      (`TextRenderComponent.K2_SetText` (`self.TextRender1`) _output_get_2)
      (`TextRenderComponent.SetTextRenderColor` (`self.TextRender`) _unloadcolor)
      (`TextRenderComponent.SetTextRenderColor` (`self.TextRender1`) _unloadcolor))))