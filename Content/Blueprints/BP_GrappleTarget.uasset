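; BP_GrappleTarget is a grapple hook target that shows its state by changing the color of its sphere.
; On BeginPlay it makes a dynamic material from the sphere's material and caches the original Color parameter.
; Targeted, InReach and Hooked events set distinct highlight colors, while OutofReach and UnTargeted restore the original.
; It also reports a static grapple gameplay tag.
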(event `self.ReceiveBeginPlay`
  (bind _returnvalue (`PrimitiveComponent.CreateDynamicMaterialInstance` (`self.Sphere`) 0 (`PrimitiveComponent.GetMaterial` (`self.Sphere`) 0) "None"))
  (bind _output_get (set `self.Dynamic Material` _returnvalue))
  (bind _returnvalue_2 (`MaterialInstanceDynamic.K2_GetVectorParameterValue` _output_get "Color"))
  (set `self.Default Color` _returnvalue_2))

(event `GrappleTargetInterface.Targeted`
  (`MaterialInstanceDynamic.SetVectorParameterValue` (`self.Dynamic Material`) "Color" (struct :`R` 1.0 :`G` 0.041141 :`B` 0.031194 :`A` 1.0)))

(event `GrappleTargetInterface.InReach`
  (`MaterialInstanceDynamic.SetVectorParameterValue` (`self.Dynamic Material`) "Color" (struct :`R` 0.71875 :`G` 0.565891 :`B` 0.063639 :`A` 1.0)))

(event `GrappleTargetInterface.OutofReach`
  (`MaterialInstanceDynamic.SetVectorParameterValue` (`self.Dynamic Material`) "Color" (`self.Default Color`) :!label _label))

(event `GrappleTargetInterface.UnTargeted`
  (goto _label))

(event `GrappleTargetInterface.Hooked`
  (`MaterialInstanceDynamic.SetVectorParameterValue` (`self.Dynamic Material`) "Color" (struct :`R` 0.019408 :`B` 1.0 :`A` 1.0)))

(fn `GetGrappledGameplayTag`
  (returns (ReturnValue :type "GameplayTag Structure"))
  (return (struct :`TagName` "GrappleTarget.Static")))

(fn `UserConstructionScript`)