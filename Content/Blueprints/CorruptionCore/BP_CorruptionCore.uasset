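; Corruption core actor that loops an idle montage, plays a smacked reaction when attacked, and drives a network of connected tendrils.
; Dynamic materials display health through four parameters on the first slot and animate a normal-offset pulse on the others.
; CommonTrigger pulses the tendrils while the core is alive.
; Death spawns a Niagara effect, then timers start a timeline-driven sphere-radius material and light fade and later destroy the connected tendrils.
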(event `self.ReceiveBeginPlay`
  (set `self.InitialScale` (`SceneComponent.K2_GetComponentScale` (`self.Root`)))
  (set `self.InitialLightStrength` (`LightComponentBase.Intensity` (`self.PointLight`)))
  (`|ExecutionSequence`
    (:`then_0`
      (`self.GetDynamicMaterial`))
    (:`then_1`
      (`self.Play Idle`))))

(event `Play Idle`
  (`|PlayMontage` (`self.Mesh`) "/Game/Models/collectibles/CorruptionCore/AM_CorruptionCore_Idle.AM_CorruptionCore_Idle" :!label _label
    (:`OnBlendOut`
      (goto _label))))

(event `/Game/Blueprints/Interfaces/Interface_CommonAnimTrigger.CorruptionCorePulseTrigger`
  (bind (_direction _value) (`Timeline|SelfPulse` :!via `PlayFromStart`)
    (:`Update`
      (for (_array_element _array_index) (`self.Core_DynamicMaterial_Array`)
        (if (not (== _array_index 0))
          (`MaterialInstanceDynamic.SetScalarParameterValue` _array_element "NormalOffset" (* _value 3.0)))))))

(event `self.ReceiveTick`
  (params (DeltaSeconds :type "Float (single-precision)")))

(event `AttackInterface.Gen_ReceiveAttack_IMPL`
  (params (Dircetion :type "Vector Structure (by ref)") (Strength :type "Float (single-precision)") (AType :type "EAttackType Enum" :default "None"))
  (`|PlayMontage` (`self.Mesh`) "/Game/Models/collectibles/CorruptionCore/AM_CorruptionCore_Smacked.AM_CorruptionCore_Smacked"
    (:`OnBlendOut`
      (`self.Play Idle`))))

(event `self.HealthUpdate`
  (params (newhealth :type Integer))
  (`self.Set Core Material Health` newhealth))

(event `/Game/Blueprints/Interfaces/Interface_CommonAnimTrigger.CommonTrigger`
  (if (not (`self.Dead`))
    (`self.Activate_TendrilPulse`)))

(event `self.Death_IMPL`
  (set `self.Dead` true)
  (`NiagaraFunctionLibrary.SpawnSystemAtLocation` "/Game/Effects/NS_Jump.NS_Jump" (`self.K2_GetActorLocation`))
  (`KismetSystemLibrary.K2_SetTimerDelegate` (delegate `FadeMaterial`) 0.3)
  (`KismetSystemLibrary.K2_SetTimerDelegate` (delegate `DestroyTendrils`) 1.6))

(event `DestroyTendrils`
  (`self.DestroyConnectedTendrils`))

(event `FadeMaterial`
  (`|ExecutionSequence`
    (:`then_0`
      (bind (_direction _value) (`Timeline|Fade_Material` :!via `PlayFromStart`)
        (:`Update`
          (for _array_element (`self.Core_DynamicMaterial_Array`)
            (`MaterialInstanceDynamic.SetScalarParameterValue` _array_element "Fade_SphereRadius" (* _value (`self.Fade_Length`)))))))
    (:`then_1`
      (bind (_direction_2 _newtrack_0) (`Timeline|LightFade` :!via `PlayFromStart`)
        (:`Update`
          (`LightComponent.SetIntensity` (`self.PointLight`) (* _newtrack_0 (`self.InitialLightStrength`))))))))

(fn `Activate_TendrilPulse`
  (for _array_element (`self.ConnectedTendrils`)
    (`/Engine/EditorBlueprintResources/StandardMacros.IsValid` _array_element
      (:`Is Valid`
        (`CorruptionTendril.TendrilPulse_Start` _array_element)))))

(fn `GetDynamicMaterial`
  (bind _mesh (`self.Mesh`))
  (bind _mesh_2 (`self.Mesh`))
  (bind _mesh_3 (`self.Mesh`))
  (bind _returnvalue (`PrimitiveComponent.CreateDynamicMaterialInstance` _mesh_2 0 (`PrimitiveComponent.GetMaterial` _mesh_2 0) "None"))
  (`KismetArrayLibrary.Array_Add` (`self.Core_DynamicMaterial_Array`) _returnvalue)
  (bind _returnvalue_2 (`PrimitiveComponent.CreateDynamicMaterialInstance` _mesh_3 1 (`PrimitiveComponent.GetMaterial` _mesh_3 1) "None"))
  (`KismetArrayLibrary.Array_Add` (`self.Core_DynamicMaterial_Array`) _returnvalue_2)
  (bind _returnvalue_3 (`PrimitiveComponent.CreateDynamicMaterialInstance` _mesh 2 (`PrimitiveComponent.GetMaterial` _mesh 2) "None"))
  (`KismetArrayLibrary.Array_Add` (`self.Core_DynamicMaterial_Array`) _returnvalue_3))

(fn `Set Core Material Health`
  (params (newHealth :type Integer))
  (locals (Core_DynamicMaterial :type "MaterialInstanceDynamic Object Reference"))
  (set `local.Core_DynamicMaterial` (`|GetArrayItem` (`self.Core_DynamicMaterial_Array`)))
  (switch `int` newHealth
    (:`0`
      (`MaterialInstanceDynamic.SetScalarParameterValue` (`local.Core_DynamicMaterial`) "Health_1" 0.0)
      (`MaterialInstanceDynamic.SetScalarParameterValue` (`local.Core_DynamicMaterial`) "Health_2" 0.0)
      (`MaterialInstanceDynamic.SetScalarParameterValue` (`local.Core_DynamicMaterial`) "Health_3" 0.0)
      (`MaterialInstanceDynamic.SetScalarParameterValue` (`local.Core_DynamicMaterial`) "Health_4" 0.0))
    (:`1`
      (`MaterialInstanceDynamic.SetScalarParameterValue` (`local.Core_DynamicMaterial`) "Health_1" 1.0)
      (`MaterialInstanceDynamic.SetScalarParameterValue` (`local.Core_DynamicMaterial`) "Health_2" 0.0)
      (`MaterialInstanceDynamic.SetScalarParameterValue` (`local.Core_DynamicMaterial`) "Health_3" 0.0)
      (`MaterialInstanceDynamic.SetScalarParameterValue` (`local.Core_DynamicMaterial`) "Health_4" 0.0))
    (:`2`
      (`MaterialInstanceDynamic.SetScalarParameterValue` (`local.Core_DynamicMaterial`) "Health_1" 1.0)
      (`MaterialInstanceDynamic.SetScalarParameterValue` (`local.Core_DynamicMaterial`) "Health_2" 1.0)
      (`MaterialInstanceDynamic.SetScalarParameterValue` (`local.Core_DynamicMaterial`) "Health_3" 0.0)
      (`MaterialInstanceDynamic.SetScalarParameterValue` (`local.Core_DynamicMaterial`) "Health_4" 0.0))
    (:`3`
      (`MaterialInstanceDynamic.SetScalarParameterValue` (`local.Core_DynamicMaterial`) "Health_1" 1.0)
      (`MaterialInstanceDynamic.SetScalarParameterValue` (`local.Core_DynamicMaterial`) "Health_2" 1.0)
      (`MaterialInstanceDynamic.SetScalarParameterValue` (`local.Core_DynamicMaterial`) "Health_3" 1.0)
      (`MaterialInstanceDynamic.SetScalarParameterValue` (`local.Core_DynamicMaterial`) "Health_4" 0.0))
    (:`4`
      (`MaterialInstanceDynamic.SetScalarParameterValue` (`local.Core_DynamicMaterial`) "Health_1" 1.0)
      (`MaterialInstanceDynamic.SetScalarParameterValue` (`local.Core_DynamicMaterial`) "Health_2" 1.0)
      (`MaterialInstanceDynamic.SetScalarParameterValue` (`local.Core_DynamicMaterial`) "Health_3" 1.0)
      (`MaterialInstanceDynamic.SetScalarParameterValue` (`local.Core_DynamicMaterial`) "Health_4" 1.0))))

(fn `UserConstructionScript`)