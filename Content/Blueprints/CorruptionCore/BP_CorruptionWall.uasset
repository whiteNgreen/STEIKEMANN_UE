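; Corruption wall actor built from four animated tendril meshes and a point light, which dies and disappears when opened.
; On BeginPlay it creates dynamic materials for the tendrils and randomizes each idle animation's start position to vary their motion.
; OpenWallImpl runs once, triggering death animations, timelines that drive a material sphere-radius fade and the light intensity, and a short lifespan.
; A separate MeatWallPulse event drives material pulse strength through a timeline.
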(event `self.ReceiveBeginPlay`
  (`self.GetDynamicMaterial`)
  (`self.SetAnimStartPosition`)
  (set `self.InitialLightIntensity` (`LightComponentBase.Intensity` (`self.PointLight`))))

(event `FadeLight`
  (bind (_direction _value) (`Timeline|FadeLight_Timeline` :!via `PlayFromStart`)
    (:`Update`
      (`LightComponent.SetIntensity` (`self.PointLight`) (* _value (`self.InitialLightIntensity`))))))

(event `self.OpenWall_Impl`
  (if (not (`self.Dead`))
    (set `self.Dead` true)
    (`self.DeathAnim`)
    (`self.SetLifeSpan` 4.1)
    (`self.FadeMaterial`)
    (`self.FadeLight`)))

(event `FadeMaterial`
  (bind (_direction _fadevalue) (`Timeline|Fade` :!via `PlayFromStart`)
    (:`Update`
      (for _array_element (`self.DynMaterials`)
        (`MaterialInstanceDynamic.SetScalarParameterValue` _array_element "Fade_SphereRadius" (* _fadevalue (`self.FadeLength`)))))))

(event `self.MeatWall_Pulse`
  (bind (_direction _value) (`Timeline|WallPulse` :!via `PlayFromStart`)
    (:`Update`
      (for _array_element (`self.DynMaterials`)
        (`MaterialInstanceDynamic.SetScalarParameterValue` _array_element "In_PulseStrength" _value)))))

(fn `DeathAnim`
  (bind _asanim_bp_tendril_wall_1 (cast `/Game/Animation/StaticObjectsAnimBP/AnimBP_TendrilWall1` (`SkeletalMeshComponent.GetAnimInstance` (`self.TW_Thick_1`))))
  (set `/Game/Animation/StaticObjectsAnimBP/AnimBP_TendrilWall1.bDeath` true _asanim_bp_tendril_wall_1)
  (bind _asanim_bp_tendril_wall_1_2 (cast `/Game/Animation/StaticObjectsAnimBP/AnimBP_TendrilWall1` (`SkeletalMeshComponent.GetAnimInstance` (`self.TW_Thick_2`))))
  (set `/Game/Animation/StaticObjectsAnimBP/AnimBP_TendrilWall1.bDeath` true _asanim_bp_tendril_wall_1_2)
  (bind _asanim_bp_tendril_wall_2 (cast `/Game/Animation/StaticObjectsAnimBP/AnimBP_TendrilWall2` (`SkeletalMeshComponent.GetAnimInstance` (`self.TW_Tangled_1`))))
  (set `/Game/Animation/StaticObjectsAnimBP/AnimBP_TendrilWall2.bDeath` true _asanim_bp_tendril_wall_2)
  (bind _asanim_bp_tendril_wall_2_2 (cast `/Game/Animation/StaticObjectsAnimBP/AnimBP_TendrilWall2` (`SkeletalMeshComponent.GetAnimInstance` (`self.TW_Tangled_2`))))
  (set `/Game/Animation/StaticObjectsAnimBP/AnimBP_TendrilWall2.bDeath` true _asanim_bp_tendril_wall_2_2))

(fn `GetDynamicMaterial`
  (bind _tw_thick_2 (`self.TW_Thick_2`))
  (bind _tw_tangled_2 (`self.TW_Tangled_2`))
  (bind _tw_tangled_1 (`self.TW_Tangled_1`))
  (bind _tw_thick_1 (`self.TW_Thick_1`))
  (`|ExecutionSequence`
    (:`then_0`
      (bind _returnvalue (`PrimitiveComponent.CreateDynamicMaterialInstance` _tw_thick_2 0 (`PrimitiveComponent.GetMaterial` _tw_thick_2 0) "None"))
      (`KismetArrayLibrary.Array_Add` (`self.DynMaterials`) _returnvalue))
    (:`then_1`
      (bind _returnvalue_2 (`PrimitiveComponent.CreateDynamicMaterialInstance` _tw_tangled_1 0 (`PrimitiveComponent.GetMaterial` _tw_tangled_1 0) "None"))
      (`KismetArrayLibrary.Array_Add` (`self.DynMaterials`) _returnvalue_2))
    (:`then_2`
      (bind _returnvalue_3 (`PrimitiveComponent.CreateDynamicMaterialInstance` _tw_tangled_2 0 (`PrimitiveComponent.GetMaterial` _tw_tangled_2 0) "None"))
      (`KismetArrayLibrary.Array_Add` (`self.DynMaterials`) _returnvalue_3))
    (:`then_3`
      (bind _returnvalue_4 (`PrimitiveComponent.CreateDynamicMaterialInstance` _tw_thick_1 0 (`PrimitiveComponent.GetMaterial` _tw_thick_1 0) "None"))
      (`KismetArrayLibrary.Array_Add` (`self.DynMaterials`) _returnvalue_4))))

(fn `SetAnimStartPosition`
  (locals (RandRange :type "Float (double-precision)" :default 1.0))
  (bind _asanim_bp_tendril_wall_1 (cast `/Game/Animation/StaticObjectsAnimBP/AnimBP_TendrilWall1` (`SkeletalMeshComponent.GetAnimInstance` (`self.TW_Thick_1`))))
  (set `/Game/Animation/StaticObjectsAnimBP/AnimBP_TendrilWall1.IdleStartPosition` (`KismetMathLibrary.RandomFloatInRange` 0.0 (`local.RandRange`)) _asanim_bp_tendril_wall_1)
  (bind _asanim_bp_tendril_wall_1_2 (cast `/Game/Animation/StaticObjectsAnimBP/AnimBP_TendrilWall1` (`SkeletalMeshComponent.GetAnimInstance` (`self.TW_Thick_2`))))
  (set `/Game/Animation/StaticObjectsAnimBP/AnimBP_TendrilWall1.IdleStartPosition` (`KismetMathLibrary.RandomFloatInRange` 0.0 (`local.RandRange`)) _asanim_bp_tendril_wall_1_2)
  (bind _asanim_bp_tendril_wall_2 (cast `/Game/Animation/StaticObjectsAnimBP/AnimBP_TendrilWall2` (`SkeletalMeshComponent.GetAnimInstance` (`self.TW_Tangled_1`))))
  (set `/Game/Animation/StaticObjectsAnimBP/AnimBP_TendrilWall2.IdleStartPosition` (`KismetMathLibrary.RandomFloatInRange` 0.0 (`local.RandRange`)) _asanim_bp_tendril_wall_2)
  (bind _asanim_bp_tendril_wall_2_2 (cast `/Game/Animation/StaticObjectsAnimBP/AnimBP_TendrilWall2` (`SkeletalMeshComponent.GetAnimInstance` (`self.TW_Tangled_2`))))
  (set `/Game/Animation/StaticObjectsAnimBP/AnimBP_TendrilWall2.IdleStartPosition` (`KismetMathLibrary.RandomFloatInRange` 0.0 (`local.RandRange`)) _asanim_bp_tendril_wall_2_2))

(fn `UserConstructionScript`)