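; BP_LevelTransition is a trigger volume that loads another level when the tagged player character enters it.
; Box overlap requires the Pottit gameplay tag and a capsule component, so other components on that actor do not set it off.
; It then shows WGT_LevelTransition with a start delay and fade speed, waits the combined start and end delays, and opens the referenced Level.
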(event `self.Box.OnComponentBeginOverlap`
  (params (OverlappedComponent :type "PrimitiveComponent Object Reference") (OtherActor :type "Actor Object Reference") (OtherComp :type "PrimitiveComponent Object Reference") (OtherBodyIndex :type Integer) (bFromSweep :type Boolean) (SweepResult :type "HitResult Structure (by ref)"))
  (bind _delaytime_start (`self.DelayTime_Start`))
  (bind _tagcontainer (message `GameplayTagAssetInterface.GetOwnedGameplayTags` OtherActor))
  (if (and (`BlueprintGameplayTagLibrary.HasTag` _tagcontainer (struct :`TagName` "Pottit") true) (`KismetMathLibrary.ClassIsChildOf` (`GameplayStatics.GetObjectClass` OtherComp) "/Script/Engine.CapsuleComponent"))
    (bind _returnvalue (`|CreateWidget` "/Game/Widget/WGT_LevelTransition.WGT_LevelTransition_C" (`GameplayStatics.GetPlayerController` 0)))
    (`UserWidget.AddToViewport` _returnvalue 0)
    (`/Game/Widget/WGT_LevelTransition.StartEvent` _returnvalue _delaytime_start 1.0)
    (`KismetSystemLibrary.Delay` (+ _delaytime_start (`self.DelayTime_End`)))
    (`GameplayStatics.OpenLevelBySoftObjectPtr` (`self.Level`))))

(fn `UserConstructionScript`)