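; Static grapple target actor, a flower that signals its grapple state to the player through glow and animation.
; On BeginPlay it replaces the flower mesh's materials with dynamic instances and caches them.
; GrappleTargetInterface events for in reach, targeted, hooked, untargeted and out of reach push emissive and fresnel presets to those materials.
; Being hooked also plays a squish montage, and the grappled tag reports GrappleTarget.Static.
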(event `self.ReceiveBeginPlay`
  (`self.CreateDynamicMaterials`))

(event `GrappleTargetInterface.Targeted`
  (`self.SetMaterialParameters` (struct :`R` 1.0 :`G` 1.0 :`B` 1.0 :`A` 1.0) 1.0 30.0 (struct :`R` 1.0 :`G` 0.773376 :`B` 0.7993 :`A` 1.0) 0.4))

(event `GrappleTargetInterface.Hooked`
  (`self.SetMaterialParameters` (struct :`R` 1.0 :`G` 1.0 :`B` 1.0 :`A` 1.0) 0.6 30.0 (struct :`R` 0.102066 :`G` 0.084354 :`B` 1.0 :`A` 1.0) 0.7)
  (`|PlayMontage` (`self.flower`) "/Game/Models/Environment/grapple/Montages/AM_GrappleTarget_Squished.AM_GrappleTarget_Squished"))

(event `GrappleTargetInterface.InReach`
  (`self.SetMaterialParameters` (struct :`R` 1.0 :`G` 1.0 :`B` 1.0 :`A` 1.0) 0.2 10.0 (struct :`R` 1.0 :`G` 1.0 :`B` 0.183333 :`A` 1.0) 0.9))

(event `GrappleTargetInterface.OutofReach`
  (`self.SetMaterialParameters` (struct :`R` 1.0 :`G` 1.0 :`B` 1.0 :`A` 1.0) 0.1 0.0 (struct :`A` 1.0) 1.0 :!label _label))

(event `GrappleTargetInterface.UnTargeted`
  (goto _label))

(fn `CreateDynamicMaterials`
  (for _array_element (`MeshComponent.GetMaterials` (`self.flower`))
    (bind _returnvalue (`KismetMaterialLibrary.CreateDynamicMaterialInstance` _array_element))
    (bind _returnvalue_2 (`KismetArrayLibrary.Array_Add` (`self.Dynamic Material`) _returnvalue))
    (`PrimitiveComponent.SetMaterial` (`self.flower`) _returnvalue_2 _returnvalue)))

(fn `GetGrappledGameplayTag`
  (returns (ReturnValue :type "GameplayTag Structure"))
  (return (struct :`TagName` "GrappleTarget.Static")))

(fn `SetMaterialParameters`
  (params (BaseColorMulti :type "LinearColor Structure" :default (struct :`R` 1.0 :`G` 1.0 :`B` 1.0 :`A` 1.0)) (EmissiveBaseColor :type "Float (double-precision)") (Emissive :type "Float (double-precision)") (`Emissive Color` :type "LinearColor Structure") (`Fresnel Threshhold` :type "Float (double-precision)"))
  (for _array_element (`self.Dynamic Material`)
    (`|ExecutionSequence`
      (:`then_0`
        (`MaterialInstanceDynamic.SetScalarParameterValue` _array_element "Emissive BaseColor" EmissiveBaseColor))
      (:`then_1`
        (`MaterialInstanceDynamic.SetScalarParameterValue` _array_element "Emissive Targeting" Emissive))
      (:`then_2`
        (`MaterialInstanceDynamic.SetVectorParameterValue` _array_element "EmissiveColor" `Emissive Color`))
      (:`then_3`
        (`MaterialInstanceDynamic.SetScalarParameterValue` _array_element "Fresnel Threshhold" `Fresnel Threshhold`))
      (:`then_4`
        (`MaterialInstanceDynamic.SetVectorParameterValue` _array_element "Color Multiplier" BaseColorMulti)))))

(fn `UserConstructionScript`)