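; Scripted dialogue prompt in which Orange Girl, a child actor, asks the player (Pottit) for 100 saps and hints at clearing roots.
; PromptChange switches on prompt index to print typewriter lines, set the speaker and drive her animations.
; The player's sap state, sampled at the first line, branches the ending between refusals and taking saps.
; Tick lerps the player camera to the prompt camera until the player leaves.
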(event `self.ReceiveBeginPlay`
  (`parent.ReceiveBeginPlay`)
  (bind _asorange_girl_character (cast `OrangeGirlCharacter` (`ChildActorComponent.ChildActor` (`self.ChildActor`))))
  (set `self.OrangeGirl` _asorange_girl_character))

(event `self.ReceiveTick`
  (params (DeltaSeconds :type "Float (single-precision)"))
  (`parent.ReceiveTick` DeltaSeconds)
  (`self.CameraLerp` DeltaSeconds))

(event `self.GetNextPromptState`
  (params (player :type "SteikemannCharacter Object Reference") (promptIndex :type Integer)))

(event `self.PromptChange`
  (bind _text_typewriterspeed (`self.Text_TypeWriterSpeed`))
  (bind _text_typewriterspeed_2 (`self.Text_TypeWriterSpeed`))
  ;[1 1 1] Prompt Switch
  (set `self.CameraLerpAlpha` 0.0)
  (switch `int` (`self.m_PromptIndex_Internal`)
    (:`0`
      ;[1 1 1] Prompt 0
      (`UserWidget.AddToViewport` (`self.DialogueWidget`) 0)
      (`self.Print Text` "ooo,  well!  Look  who  it  is." false (`self.Text_TypeWriterSpeed`))
      (`OrangeGirlCharacter.Anim_State` (`self.OrangeGirl`) "ClutchStomach")
      (set `self.Enum_CameraLerp` "First")
      (bind _returnvalue (`SteikemannCharacter.GetLoseSapType` (`self.m_Player`)))
      (set `self.LoseSapType` _returnvalue)
      (set `SteikemannCharacter.bInPrompt` true (`self.m_Player`))
      (`SceneComponent.SetVisibility` (`self.Button`) false false)
      (`SceneComponent.SetVisibility` (`self.ExclamationPoint`) false false)
      (`/Game/Widget/DialoguePrompt/WGT_DialogueBox.Owner_OrangeGirl` (`self.DialogueWidget`)))
    (:`1`
      ;[1 1 1] Prompt 1
      (`self.Print Text` "You  again!  How... \nHow  did  you  get  here  before  me!? \n........... \n....What's  wrong?" true (`self.Text_TypeWriterSpeed`))
      (`OrangeGirlCharacter.Anim_State` (`self.OrangeGirl`) "ClutchStomach")
      (`/Game/Widget/DialoguePrompt/WGT_DialogueBox.Owner_Pottit` (`self.DialogueWidget`)))
    (:`2`
      ;[1 1 1] Prompt 2
      (`self.Print Text` "Owh...My  stomach  hurts,  must be one  one  of  those   \ndragon  fruit  slices  I  ate.  Or  maybe  it's  the   \nweird  smell  from  those  red  roots." true (`self.Text_TypeWriterSpeed`))
      (`OrangeGirlCharacter.Anim_State` (`self.OrangeGirl`) "BobUpDown")
      (`/Game/Widget/DialoguePrompt/WGT_DialogueBox.Owner_OrangeGirl` (`self.DialogueWidget`)))
    (:`3`
      (`self.Print Text` "How  about...  you  give  me  100  saps? \nI'm  SURE  I'll  feel  better  then." true (`self.Text_TypeWriterSpeed`))
      (`OrangeGirlCharacter.Anim_State` (`self.OrangeGirl`) "NeedSaps")
      (`/Game/Widget/DialoguePrompt/WGT_DialogueBox.Owner_OrangeGirl` (`self.DialogueWidget`)))
    (:`4`
      (`self.Print Text` "What?  How  are  saps  going  to  help  \nwith  that?" true (`self.Text_TypeWriterSpeed`))
      (`OrangeGirlCharacter.Anim_State` (`self.OrangeGirl`) "NeedSaps")
      (`/Game/Widget/DialoguePrompt/WGT_DialogueBox.Owner_Pottit` (`self.DialogueWidget`)))
    (:`5`
      ;[1 1 1] Prompt 3
      (`self.Print Text` "Hey,  don't  think  too  hard  about  it. \nJust  give  me  100  of  them.  \nYou'd  be,  like,  my  hero." false (`self.Text_TypeWriterSpeed`))
      (`OrangeGirlCharacter.Anim_State` (`self.OrangeGirl`) "GiveSapsPlz")
      (`/Game/Widget/DialoguePrompt/WGT_DialogueBox.Owner_OrangeGirl` (`self.DialogueWidget`)))
    (:`6`
      ;[1 1 1] Prompt 3
      (`self.Print Text` "On  that  note,  seems  like  those  evil  roots  are   \nblocking  the  way  out  of  the  cliff too.   \nSounds  like  a  job  for  a  hero,  no?" false (`self.Text_TypeWriterSpeed`))
      (`OrangeGirlCharacter.Anim_State` (`self.OrangeGirl`) "GiveSapsPlz")
      (`/Game/Widget/DialoguePrompt/WGT_DialogueBox.Owner_OrangeGirl` (`self.DialogueWidget`)))
    (:`7`
      (`self.Print Text` "Okay  fine!  I'll  give  you  your  saps!   \nBut  when  I've  cleared  the  suspicious  roots, \nyou  better  not  follow  me  young  lady!" true (`self.Text_TypeWriterSpeed`))
      (`OrangeGirlCharacter.Anim_State` (`self.OrangeGirl`) "NeedSaps")
      (`/Game/Widget/DialoguePrompt/WGT_DialogueBox.Owner_Pottit` (`self.DialogueWidget`)))
    (:`8`
      (`self.Print Text` "Yeah,  sure  thing  mr.  hero \nThanks  a  bunch." false (`self.Text_TypeWriterSpeed`))
      (`OrangeGirlCharacter.Anim_State` (`self.OrangeGirl`) "GiveSapsPlz")
      (`/Game/Widget/DialoguePrompt/WGT_DialogueBox.Owner_OrangeGirl` (`self.DialogueWidget`)))
    (:`9`
      ;[1 1 1] Prompt 4
      (switch `ELoseSapType` (`self.LoseSapType`)
        (:`PlayerHasNoSaps`
          (`self.Print Text` "What! I see  you  only  have  like,  0 !? " false _text_typewriterspeed)
          (`OrangeGirlCharacter.Anim_State` (`self.OrangeGirl`) "BobUpDown")
          (`/Game/Widget/DialoguePrompt/WGT_DialogueBox.Owner_OrangeGirl` (`self.DialogueWidget`)))
        (:`PlayerHasNotEnough`
          (`self.Print Text` "Oh  NO!  I  see  you  don't  have   nearly  enough! \nI  need  100 saps.  For  my  stomach." false _text_typewriterspeed)
          (`OrangeGirlCharacter.Anim_State` (`self.OrangeGirl`) "ClutchStomach")
          (`/Game/Widget/DialoguePrompt/WGT_DialogueBox.Owner_OrangeGirl` (`self.DialogueWidget`)))
        (:`LoseAllSaps`
          (`self.Print Text` "Would  you  look  at  that,  you  got  me  100! \nThanks!  I  had  my  doubts  there.  But  I  guess  you   \nreally  are  a  hero.  I  suppose  I'll  be  on  my  way  now, \nlike  you  told  me  to." true _text_typewriterspeed)
          (`SteikemannCharacter.LoseSaps` (`self.m_Player`) -1))))
    (:`10`
      ;[1 1 1] Prompt 5
      (switch `ELoseSapType` (`self.LoseSapType`)
        (:`PlayerHasNoSaps`
          (`self.Print Text` "Come  back  when  you've  got  more.  \nI'd  rather  get  going  soon.    \nUgh. \nMaybe  the  smell  has  infiltrated  my  endocarp..." true _text_typewriterspeed_2)
          (`OrangeGirlCharacter.Anim_State` (`self.OrangeGirl`) "BobUpDown")
          (`/Game/Widget/DialoguePrompt/WGT_DialogueBox.Owner_OrangeGirl` (`self.DialogueWidget`)))
        (:`PlayerHasNotEnough`
          (`self.Print Text` "Please  come  back  with  more. \nMy  town  is  beyond  this  cliff,   \nand  I  can't get  over  it  in  this  sorry  state,   \ncan  I? " false _text_typewriterspeed_2)
          (`OrangeGirlCharacter.Anim_State` (`self.OrangeGirl`) "ClutchStomach")
          (`/Game/Widget/DialoguePrompt/WGT_DialogueBox.Owner_OrangeGirl` (`self.DialogueWidget`)))
        (:`LoseAllSaps`
          (`self.PlayerLeavesPrompt`))))
    (:`11`
      ;[1 1 1] Prompt 6
      (switch `ELoseSapType` (`self.LoseSapType`)
        (:`PlayerHasNoSaps`
          _)
        (:`PlayerHasNotEnough`
          _)
        (:`LoseAllSaps`
          _))
      (`self.PlayerLeavesPrompt`))))

(fn `CameraLerp`
  (params (DeltaTime :type "Float (double-precision)"))
  (`parent.CameraLerp` DeltaTime)
  (switch `ECameraLerp` (`self.Enum_CameraLerp`)
    (:`First`
      (bind _returnvalue (`self.LerpSceneComponentTransformToSceneComponent` (`self.m_PlayerCamera`) (`self.Camera`) (`self.CameraLerpAlpha`) DeltaTime))
      (set `self.CameraLerpAlpha` _returnvalue))))

(fn `On_ExitPrompt`
  (`parent.On_ExitPrompt`)
  (`OrangeGirlCharacter.Anim_State` (`self.OrangeGirl`) "Idle"))

(fn `PlayerLeavesPrompt`
  (set `self.Enum_CameraLerp` "None")
  (set `SteikemannCharacter.bInPrompt` false (`self.m_Player`))
  (`self.ExitPrompt` 0.0))

(fn `UserConstructionScript`
  (`parent.UserConstructionScript`))