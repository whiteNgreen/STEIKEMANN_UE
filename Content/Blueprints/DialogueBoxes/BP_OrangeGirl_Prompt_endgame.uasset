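; Endgame dialogue prompt Blueprint for the Orange Girl NPC, playing a scripted conversation between her and the player character Pottit.
; PromptChange switches on the prompt index, printing typewriter text, setting the speaker on the dialogue widget and Orange Girl's animation, until the last index exits the prompt.
; Tick lerps the player camera to the prompt camera while the conversation runs.
; Older sap-payment branches remain but are disconnected.
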(event `self.ReceiveBeginPlay`
  (`parent.ReceiveBeginPlay`)
  (bind _asorange_girl_character (cast `OrangeGirlCharacter` (`ChildActorComponent.ChildActor` (`self.ChildActor`))))
  (set `self.OrangeGirl` _asorange_girl_character))

(event `self.ReceiveTick`
  (params (DeltaSeconds :type "Float (single-precision)"))
  (`parent.ReceiveTick` DeltaSeconds)
  (`self.CameraLerp` DeltaSeconds))

(event `self.GetNextPromptState`
  (params (player :type "SteikemannCharacter Object Reference") (promptIndex :type Integer)))

(event `self.PromptChange`
  ;[1 1 1] Prompt Switch
  (set `self.CameraLerpAlpha` 0.0)
  (switch `int` (`self.m_PromptIndex_Internal`)
    (:`0`
      ;[1 1 1] Prompt 0
      (`UserWidget.AddToViewport` (`self.DialogueWidget`) 0)
      (`self.Print Text` "Oh, Hi..." false (`self.Text_TypeWriterSpeed`))
      (`OrangeGirlCharacter.Anim_State` (`self.OrangeGirl`) "Idle")
      (set `self.Enum_CameraLerp` "First")
      (bind _returnvalue (`SteikemannCharacter.GetLoseSapType` (`self.m_Player`)))
      (set `self.LoseSapType` _returnvalue)
      (set `SteikemannCharacter.bInPrompt` true (`self.m_Player`))
      (`SceneComponent.SetVisibility` (`self.Button`) false false)
      (`SceneComponent.SetVisibility` (`self.ExclamationPoint`) false false)
      (`/Game/Widget/DialoguePrompt/WGT_DialogueBox.Owner_OrangeGirl` (`self.DialogueWidget`)))
    (:`1`
      ;[1 1 1] Prompt 1
      (`self.Print Text` "It's  been  a  while  since  I've  traveled  home. \nBut  I don't  remember  seeing  anything  like  this." true (`self.Text_TypeWriterSpeed`))
      (`OrangeGirlCharacter.Anim_State` (`self.OrangeGirl`) "Idle"))
    (:`2`
      ;[1 1 1] Prompt 2
      (`self.Print Text` "How  di-... Never  mind. \nYeah,  this  certainly  took  a turn. \nCan't  say  I've  seen  mushrooms  like  these \nbefore  either." true (`self.Text_TypeWriterSpeed`))
      (`OrangeGirlCharacter.Anim_State` (`self.OrangeGirl`) "Idle")
      (`/Game/Widget/DialoguePrompt/WGT_DialogueBox.Owner_Pottit` (`self.DialogueWidget`)))
    (:`3`
      (`self.Print Text` "Anyway,  how's  your  stomach?" true (`self.Text_TypeWriterSpeed`))
      (`OrangeGirlCharacter.Anim_State` (`self.OrangeGirl`) "Idle")
      (`/Game/Widget/DialoguePrompt/WGT_DialogueBox.Owner_Pottit` (`self.DialogueWidget`)))
    (:`4`
      ;[1 1 1] Prompt 3
      (`self.Print Text` "Oh,  I  lied. \nI  need  saps  to  pay  for  a  ferry  across \nthe  river.  If  there  even  is  a  river  anymore. \nI  don't  think  these  are  mushrooms,   mr.  hero." false (`self.Text_TypeWriterSpeed`))
      (`OrangeGirlCharacter.Anim_State` (`self.OrangeGirl`) "Idle")
      (`/Game/Widget/DialoguePrompt/WGT_DialogueBox.Owner_OrangeGirl` (`self.DialogueWidget`)))
    (:`5`
      ;[1 1 1] Prompt 3
      (`self.Print Text` "....  \nI  am  just  going  to  ignore  that  first  part. \nWe  got  bigger  issues!  What  do  you  mean \n\"they  are  not  mushrooms\"?  \nMaybe  they're  evil  mushrooms! \n" false (`self.Text_TypeWriterSpeed`))
      (`OrangeGirlCharacter.Anim_State` (`self.OrangeGirl`) "Idle")
      (`/Game/Widget/DialoguePrompt/WGT_DialogueBox.Owner_Pottit` (`self.DialogueWidget`)))
    (:`6`
      (`self.Print Text` "I mean,  it  is  not  natural  to  our  world. \nIt  reminds  me  of  a  story  I heard  a  while  back. \nAbout  an  ancient  force,  locked  away  somewhere \non  this  island.  Maybe  it  has  finally  broken  free?" true (`self.Text_TypeWriterSpeed`))
      (`OrangeGirlCharacter.Anim_State` (`self.OrangeGirl`) "Idle")
      (`/Game/Widget/DialoguePrompt/WGT_DialogueBox.Owner_OrangeGirl` (`self.DialogueWidget`)))
    (:`7`
      ;[1 1 1] Prompt 3
      (`self.Print Text` "Prft,  I've  never  heard  of  any  such story! \nMight  as  well  be  evil  mushrooms! \n" false (`self.Text_TypeWriterSpeed`))
      (`OrangeGirlCharacter.Anim_State` (`self.OrangeGirl`) "Idle")
      (`/Game/Widget/DialoguePrompt/WGT_DialogueBox.Owner_Pottit` (`self.DialogueWidget`)))
    (:`8`
      (`self.Print Text` "Whatever  it  is,  I  am  going  home! \nI  need  to  see...I  just  need  to  go." true (`self.Text_TypeWriterSpeed`))
      (`OrangeGirlCharacter.Anim_State` (`self.OrangeGirl`) "Idle")
      (`/Game/Widget/DialoguePrompt/WGT_DialogueBox.Owner_OrangeGirl` (`self.DialogueWidget`)))
    (:`9`
      (`self.Print Text` "Oh,  well  fine!   \nBut  I  cannot  possibly  let  you  go \nunsupervised  into  what  gross   \nsticky  mess  this  is  shaping  up  to  be!  I'll  keep  my   \neye  on  you.  And  my  leek  ready  for  danger!" false (`self.Text_TypeWriterSpeed`))
      (`OrangeGirlCharacter.Anim_State` (`self.OrangeGirl`) "Idle")
      (`/Game/Widget/DialoguePrompt/WGT_DialogueBox.Owner_Pottit` (`self.DialogueWidget`)))
    (:`10`
      (`self.Print Text` "Gee  thanks,  I  feel  much  safer  now. \nYou  know... For  a  disgusting  and  sticky  place, \nThat  flower  over  there  sure  is  beautiful. \nI  wonder  how  it  can  still  bloom  in  a  place   \nlike  this." true (`self.Text_TypeWriterSpeed`))
      (`OrangeGirlCharacter.Anim_State` (`self.OrangeGirl`) "Idle")
      (`/Game/Widget/DialoguePrompt/WGT_DialogueBox.Owner_OrangeGirl` (`self.DialogueWidget`)))
    (:`11`
      (`self.PlayerLeavesPrompt`))))

(fn `CameraLerp`
  (params (DeltaTime :type "Float (double-precision)"))
  (`parent.CameraLerp` DeltaTime)
  (switch `ECameraLerp` (`self.Enum_CameraLerp`)
    (:`First`
      (bind _returnvalue (`self.LerpSceneComponentTransformToSceneComponent` (`self.m_PlayerCamera`) (`self.Camera`) (`self.CameraLerpAlpha`) DeltaTime))
      (set `self.CameraLerpAlpha` _returnvalue))))

(fn `On_ExitPrompt`
  (`parent.On_ExitPrompt`)
  (`OrangeGirlCharacter.Anim_State` (`self.OrangeGirl`) "Idle"))

(fn `PlayerLeavesPrompt`
  (set `self.Enum_CameraLerp` "None")
  (set `SteikemannCharacter.bInPrompt` false (`self.m_Player`))
  (`self.ExitPrompt` 0.0))

(fn `UserConstructionScript`
  (`parent.UserConstructionScript`))