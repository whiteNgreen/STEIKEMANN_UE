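; Tutorial dialogue prompt that plays a scripted argument between the Orange Girl NPC and the player's hero, Pottit.
; PromptChange switches on the parent's prompt index to print typewriter lines, set the speaker and animate the child-actor Orange Girl.
; Tick lerps the player camera toward the prompt camera until the final step exits the prompt.
; Sap-payment branches remain but are disconnected, though the sap type is still fetched.
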(event `self.ReceiveBeginPlay`
  (`parent.ReceiveBeginPlay`)
  (bind _asorange_girl_character (cast `OrangeGirlCharacter` (`ChildActorComponent.ChildActor` (`self.ChildActor`))))
  (set `self.OrangeGirl` _asorange_girl_character))

(event `self.ReceiveTick`
  (params (DeltaSeconds :type "Float (single-precision)"))
  (`parent.ReceiveTick` DeltaSeconds)
  (`self.CameraLerp` DeltaSeconds))

(event `self.GetNextPromptState`
  (params (player :type "SteikemannCharacter Object Reference") (promptIndex :type Integer)))

(event `self.PromptChange`
  ;[1 1 1] Prompt Switch
  (set `self.CameraLerpAlpha` 0.0)
  (switch `int` (`self.m_PromptIndex_Internal`)
    (:`0`
      ;[1 1 1] Prompt 0
      (`UserWidget.AddToViewport` (`self.DialogueWidget`) 0)
      (`self.Print Text` "Huh, what?  you  are  that  one  rich  guy,  \nfrom  down  town  right?" false (`self.Text_TypeWriterSpeed`))
      (`OrangeGirlCharacter.Anim_State` (`self.OrangeGirl`) "Idle")
      (set `self.Enum_CameraLerp` "First")
      (bind _returnvalue (`SteikemannCharacter.GetLoseSapType` (`self.m_Player`)))
      (set `self.LoseSapType` _returnvalue)
      (set `SteikemannCharacter.bInPrompt` true (`self.m_Player`))
      (`SceneComponent.SetVisibility` (`self.Button`) false false)
      (`SceneComponent.SetVisibility` (`self.ExclamationPoint`) false false)
      (`/Game/Widget/DialoguePrompt/WGT_DialogueBox.Owner_OrangeGirl` (`self.DialogueWidget`)))
    (:`1`
      ;[1 1 1] Prompt 1
      (`self.Print Text` "What  are  you  doing  here?  I  heard  the  town \ntold  nobody  to  venture  out  here. " true (`self.Text_TypeWriterSpeed`))
      (`OrangeGirlCharacter.Anim_State` (`self.OrangeGirl`) "Idle"))
    (:`2`
      ;[1 1 1] Prompt 2
      (`self.Print Text` "Little Orange,  You  have  clearly  not  been   \ninformend  about  my  Quest. You  see,  I'm  on  a   \nquest  to  defeat  evil.  You  may  thank  me  now   \nfor  releasing  you  from  those  suspicious  red  \nwiggly  root  things! " true (`self.Text_TypeWriterSpeed`))
      (`OrangeGirlCharacter.Anim_State` (`self.OrangeGirl`) "Idle")
      (`/Game/Widget/DialoguePrompt/WGT_DialogueBox.Owner_Pottit` (`self.DialogueWidget`)))
    (:`3`
      (`self.Print Text` "Also,  speak  for  yourself! \nWhat  is  a  little  Orange  Girl  doing  in  these   \nOFF  LIMITS  wood  anyway!  As  a  hero  I  must \nensure  your  safity!  so  go  back  now." true (`self.Text_TypeWriterSpeed`))
      (`OrangeGirlCharacter.Anim_State` (`self.OrangeGirl`) "Idle")
      (`/Game/Widget/DialoguePrompt/WGT_DialogueBox.Owner_Pottit` (`self.DialogueWidget`)))
    (:`4`
      ;[1 1 1] Prompt 3
      (`self.Print Text` "Yeah?  well  I  am  not  going  that  way. \nI'm  on  my  way  to  the  town  behind  the  big  tree. \nAnd  I  am  not  stopping  for  anything!   \nso  don't  try  to  stop  me, \"hero\"!" false (`self.Text_TypeWriterSpeed`))
      (`OrangeGirlCharacter.Anim_State` (`self.OrangeGirl`) "Idle")
      (`/Game/Widget/DialoguePrompt/WGT_DialogueBox.Owner_OrangeGirl` (`self.DialogueWidget`)))
    (:`5`
      ;[1 1 1] Prompt 3
      (`self.Print Text` "I've  seen  you  around.   \nIf  YOU  are  tasked  with  whatever  this  \nforest  holds,  I  think  I'll  be  just  fine." false (`self.Text_TypeWriterSpeed`))
      (`OrangeGirlCharacter.Anim_State` (`self.OrangeGirl`) "GiveSapsPlz")
      (`/Game/Widget/DialoguePrompt/WGT_DialogueBox.Owner_OrangeGirl` (`self.DialogueWidget`)))
    (:`6`
      (`self.Print Text` "You  rude  little  thing!  Don't  make  me   \nuse  this  staff  to,  I  don't  know, \nGENTLY  sweep  you  back  into  town!" true (`self.Text_TypeWriterSpeed`))
      (`OrangeGirlCharacter.Anim_State` (`self.OrangeGirl`) "GiveSapsPlz")
      (`/Game/Widget/DialoguePrompt/WGT_DialogueBox.Owner_Pottit` (`self.DialogueWidget`)))
    (:`7`
      ;[1 1 1] Prompt 3
      (`self.Print Text` "Hah,  with  that  silly  thing?  Don't  make  me  laugh!  \nEveryone  knows  how  useless  that  twig  is!   \nhaha!" false (`self.Text_TypeWriterSpeed`))
      (`OrangeGirlCharacter.Anim_State` (`self.OrangeGirl`) "BobUpDown")
      (`/Game/Widget/DialoguePrompt/WGT_DialogueBox.Owner_OrangeGirl` (`self.DialogueWidget`)))
    (:`8`
      (`self.PlayerLeavesPrompt`))))

(fn `CameraLerp`
  (params (DeltaTime :type "Float (double-precision)"))
  (`parent.CameraLerp` DeltaTime)
  (switch `ECameraLerp` (`self.Enum_CameraLerp`)
    (:`First`
      (bind _returnvalue (`self.LerpSceneComponentTransformToSceneComponent` (`self.m_PlayerCamera`) (`self.Camera`) (`self.CameraLerpAlpha`) DeltaTime))
      (set `self.CameraLerpAlpha` _returnvalue))))

(fn `On_ExitPrompt`
  (`parent.On_ExitPrompt`)
  (`OrangeGirlCharacter.Anim_State` (`self.OrangeGirl`) "Idle"))

(fn `PlayerLeavesPrompt`
  (set `self.Enum_CameraLerp` "None")
  (set `SteikemannCharacter.bInPrompt` false (`self.m_Player`))
  (`self.ExitPrompt` 0.0))

(fn `UserConstructionScript`
  (`parent.UserConstructionScript`))