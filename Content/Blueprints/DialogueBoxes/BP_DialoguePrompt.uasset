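; Dialogue prompt actor that shows a button near the player and plays a short hard-coded conversation asking Potitt to investigate a red light.
; PromptChange steps by prompt index, creating WBP_DialogueBox, feeding it typewriter text, then removing it, as ExitPrompt also does.
; Tick turns the prompt toward the player camera while in range and blends that camera toward one of two enum-selected shots, with each prompt change restarting the blend.
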(event `self.ReceiveBeginPlay`
  (`SceneComponent.SetVisibility` (`self.Button`) (`self.bPlayerWithinVolume`) false))

(event `self.ReceiveTick`
  (params (DeltaSeconds :type "Float (single-precision)"))
  (`self.ButtonLookatCamera`)
  (`self.CameraLerp` DeltaSeconds))

(event `self.ShowPrompt`
  (`SceneComponent.SetVisibility` (`self.Button`) true false))

(event `self.PromptChange`
  (set `self.CameraLerpAlpha` 0.0)
  (switch `int` (`KismetMathLibrary.Conv_ByteToInt` (`self.m_PromptIndex`))
    (:`0`
      (bind _returnvalue (`|CreateWidget` "/Game/Widget/DialoguePrompt/WBP_DialogueBox.WBP_DialogueBox_C" (`GameplayStatics.GetPlayerController` 0)))
      (bind _output_get (set `self.DialogueWidget` _returnvalue))
      (`UserWidget.AddToViewport` _output_get 0)
      (`/Game/Widget/DialoguePrompt/WBP_DialogueBox.SetNewText` (`self.DialogueWidget`) "Potitt? I need your help!" (`self.Text_TypeWriterSpeed`))
      (`SceneComponent.SetVisibility` (`self.Button`) false false))
    (:`1`
      (`/Game/Widget/DialoguePrompt/WBP_DialogueBox.SetNewText` (`self.DialogueWidget`) "See The Big Tree?  \nWhat the hell is that red light?" (`self.Text_TypeWriterSpeed`)))
    (:`2`
      (`/Game/Widget/DialoguePrompt/WBP_DialogueBox.SetNewText` (`self.DialogueWidget`) "Go check it out please." (`self.Text_TypeWriterSpeed`)))
    (:`3`
      (`Widget.RemoveFromParent` (`self.DialogueWidget`) :!label _label)
      (`SceneComponent.SetVisibility` (`self.Button`) (`self.bPlayerWithinVolume`) false))))

(event `self.EndPrompt`
  (`SceneComponent.SetVisibility` (`self.Button`) false false))

(event `self.ExitPrompt`
  (goto _label))

(fn `ButtonLookatCamera`
  (bind _prompt (`self.Prompt`))
  (if (`self.bPlayerWithinVolume`)
    (`SceneComponent.K2_SetWorldTransform` _prompt (`KismetAnimationLibrary.K2_LookAt` (`SceneComponent.K2_GetComponentToWorld` _prompt) (`SceneComponent.K2_GetComponentLocation` (`self.m_PlayerCamera`)) (1.0 0.0 0.0) false (0.0 0.0 1.0)) false false)
    (`SceneComponent.K2_SetWorldRotation` _prompt (`KismetMathLibrary.MakeRotator` 0.0 (.pitch (`SceneComponent.K2_GetComponentRotation` _prompt)) (.yaw (`SceneComponent.K2_GetComponentRotation` _prompt))) false false)))

(fn `CameraLerp`
  (params (`local deltatime` :type "Float (double-precision)"))
  (locals (TargetTransform :type "Transform Structure"))
  (switch `ECameraLerp` (`self.m_ECameraLerp`)
    (:`First`
      (set `local.TargetTransform` (`SceneComponent.K2_GetComponentToWorld` (`self.Camera_One`))))
    (:`Second`
      (set `local.TargetTransform` (`SceneComponent.K2_GetComponentToWorld` (`self.Camera_Two`)))))
  (bind _output_get (set `self.CameraLerpAlpha` (`KismetMathLibrary.FClamp` (+ (`self.CameraLerpAlpha`) (* (`local.local deltatime`) (`self.CameraLerpSpeed`))))))
  (`SceneComponent.K2_SetWorldTransform` (`self.m_PlayerCamera`) (`KismetMathLibrary.TLerp` (`SceneComponent.K2_GetComponentToWorld` (`self.m_PlayerCamera`)) (`local.TargetTransform`) _output_get) false false))

(fn `UserConstructionScript`)