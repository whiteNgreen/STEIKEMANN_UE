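; Dialogue prompt actor for the NPC Gilbert, who warns the player about the glowing red tree and his grandson missing in the woods.
; PromptChange steps through the lines by prompt index, showing the dialogue widget, hiding prompt markers, toggling the player's InPrompt state and exiting at the end.
; It also picks a camera target, which Tick's CameraLerp override blends the player camera toward.
; GetNextPromptState is an obsolete, empty leftover.
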(event `self.ReceiveBeginPlay`
  (`parent.ReceiveBeginPlay`))

(event `self.ReceiveTick`
  (params (DeltaSeconds :type "Float (single-precision)"))
  (`parent.ReceiveTick` DeltaSeconds)
  (`self.CameraLerp` DeltaSeconds))

(event `self.PromptChange`
  (set `self.CameraLerpAlpha` 0.0)
  (switch `int` (`self.m_PromptIndex_Internal`)
    (:`0`
      (`UserWidget.AddToViewport` (`self.DialogueWidget`) 0)
      (`/Game/Widget/DialoguePrompt/WGT_DialogueBox.SetNewText` (`self.DialogueWidget`) "...Who?  Oh,  you  are  the  one  from \nthe  papers?  Going  out  to  investigate  are  you?   \nPottit,  was  the  name? \n" (`self.Text_TypeWriterSpeed`))
      (`SceneComponent.SetVisibility` (`self.Button`) false false)
      (`SceneComponent.SetVisibility` (`self.ExclamationPoint`) false false)
      (set `self.Enum_CameraLerp` "First")
      (set `SteikemannCharacter.bInPrompt` true (`self.m_Player`))
      (`/Game/Widget/DialoguePrompt/WGT_DialogueBox.Owner_Gilbert` (`self.DialogueWidget`)))
    (:`1`
      (`self.Print Text` "There  is  a  stange  tinge  in  the  air. \nAnd  The  great  tree  over  there  has   \nbeen  glowing  brighter  red  each day. \nI  suppose  that  is  a  place  to  start,  if  you   \nmust  go.")
      (set `self.Enum_CameraLerp` "Second"))
    (:`2`
      (`self.Print Text` "But  please  be  careful,  my  grandson   \ndissappeared  somewhere  in  those  woods  some  \nwhile  ago... I  am  afraid  that whatever \nlurks  out  there is  not  of  the  friendly  sort..."))
    (:`3`
      (`self.ExitPrompt` 0.0)
      (set `self.Enum_CameraLerp` "None")
      (set `SteikemannCharacter.bInPrompt` false (`self.m_Player`)))))

(event `self.GetNextPromptState`
  (params (player :type "SteikemannCharacter Object Reference") (promptIndex :type Integer)))

(fn `CameraLerp`
  (params (DeltaTime :type "Float (double-precision)"))
  (`parent.CameraLerp` DeltaTime)
  (switch `ECameraLerp` (`self.Enum_CameraLerp`)
    (:`First`
      (bind _returnvalue (`self.LerpSceneComponentTransformToSceneComponent` (`self.m_PlayerCamera`) (`self.Camera One`) (`self.CameraLerpAlpha`) DeltaTime))
      (set `self.CameraLerpAlpha` _returnvalue))
    (:`Second`
      (bind _returnvalue_2 (`self.LerpSceneComponentTransformToSceneComponent` (`self.m_PlayerCamera`) (`self.Camera Two`) (`self.CameraLerpAlpha`) DeltaTime))
      (set `self.CameraLerpAlpha` _returnvalue_2))))

(fn `UserConstructionScript`
  (`parent.UserConstructionScript`))