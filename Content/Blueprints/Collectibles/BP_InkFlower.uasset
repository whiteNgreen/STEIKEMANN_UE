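; BP_InkFlower is a squid-like flower that, when hit open, raises a spinning beak, spits ink and spawns an ink collectible.
; AnimOpen chains body and beak montages with timers that trigger the spawn, beak-raise timeline and Niagara ink.
; A timeline ramps rotation speed once tick is enabled, with beak and ink counter-rotating.
; Collected plays a burst effect and stops the ink.
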(event `self.ReceiveTick`
  (params (DeltaSeconds :type "Float (single-precision)"))
  (bind _returnvalue (* DeltaSeconds (`self.BeakRotationSpeed`)))
  ;[1 1 1] Tick
  (`SceneComponent.K2_AddWorldRotation` (`self.BeakMesh`) (`KismetMathLibrary.MakeRotator` 0.0 0.0 _returnvalue) false false)
  (`SceneComponent.K2_AddWorldRotation` (`self.Niagara_Ink`) (`KismetMathLibrary.MakeRotator` 0.0 0.0 (* _returnvalue -1.0)) false false))

(event `self.Anim_Hit`
  (`|PlayMontage` (`self.Mesh`) "/Game/Models/collectibles/InkFlower/Montages/AM_beakless_LightSmacked.AM_beakless_LightSmacked"))

(event `self.Anim_Open`
  (`KismetSystemLibrary.K2_SetTimerDelegate` (delegate `SpawnCollectible`) 1.5) ; Spawn Collectible
  ;[1 1 1] Beak Open
  (`KismetSystemLibrary.K2_SetTimerDelegate` (delegate `BeakOpen`) 1.0)
  ;[1 1 1] Squid Open Animation
  (`|PlayMontage` (`self.Mesh`) "/Game/Models/collectibles/InkFlower/Montages/AM_beakless_smacked.AM_beakless_smacked"
    (:`OnBlendOut`
      (`|PlayMontage` (`self.Mesh`) "/Game/Models/collectibles/InkFlower/Montages/AM_beakless_opens.AM_beakless_opens"))))

(event `BeakOpen`
  ;[1 1 1] Beak Open
  (`|PlayMontage` (`self.BeakMesh`) "/Game/Models/collectibles/InkFlower/Montages/AM_Beak_opens.AM_Beak_opens"
    (:`then`
      ;[1 1 1] Enable Beak Rotation (tick)
      (`KismetSystemLibrary.K2_SetTimerDelegate` (delegate `Enable Beak Rotation`) 0.3)
      ;[0.1927 0.1927 0.1927] Ink Particle (Spitting Out)
      (`KismetSystemLibrary.K2_SetTimerDelegate` (delegate `Ink_Particles`) 0.9))))

(event `Enable Beak Rotation`
  ;[1 1 1] Enable Beak Rotation (tick)
  (`self.SetActorTickEnabled` true)
  (bind (_direction _beakrotation_lerp) (`Timeline|Beak Rotation Strength`)
    (:`Update`
      (set `self.BeakRotationSpeed` (* _beakrotation_lerp (`self.BeakRotationSpeed_Base`))))))

(event `Ink_Particles`
  ;[0.1927 0.1927 0.1927] Ink Particle (Spitting Out)
  (if (`self.bActive`)
    (`ActorComponent.Activate` (`self.Niagara_Ink`) false)))

(event `SpawnCollectible`
  ;[1 1 1] Spawn Collectible
  (`self.SpawnInkCollectible`)
  ;[0.2314 0.2314 0.2314] Raise Beak Position
  (bind (_direction _zposition) (`Timeline|BeakPosition`)
    (:`Update`
      (`SceneComponent.K2_SetRelativeLocation` (`self.BeakMesh`) (`KismetMathLibrary.MakeVector` 0.0 0.0 _zposition) false false))))

(event `self.Collected`
  ;[1 1 1] Particle On Getting Collected
  (`NiagaraFunctionLibrary.SpawnSystemAtLocation` "/Game/Effects/NS_Jump.NS_Jump" (`SceneComponent.K2_GetComponentLocation` (`self.BeakMesh`)) (struct) (1.0 1.0 1.0) true true "AutoRelease")
  (`ActorComponent.Deactivate` (`self.Niagara_Ink`))
  (set `self.bActive` false))

(fn `UserConstructionScript`)