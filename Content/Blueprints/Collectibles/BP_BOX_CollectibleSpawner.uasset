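; Box-shaped collectible spawner that scatters child actors at random points derived from its Box component.
; The construction script adds SpawnAmount child actor components with manual attachment, each placed using GetRandomBoxLocation, so placement happens at construction rather than on BeginPlay.
; BeginPlay calls the parent and sets SpawnerComponent to the Box, while overlap and tick events are disabled stubs.
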(event `self.ReceiveBeginPlay`
  (`parent.ReceiveBeginPlay`)
  (set `self.SpawnerComponent` (`self.Box`)))

(fn `UserConstructionScript`
  (`parent.UserConstructionScript`)
  (for _ (range (`self.SpawnAmount`))
    (bind _returnvalue (`self.GetRandomBoxLocation` (`self.Box`)))
    (`AddComponent|NODE_AddChildActorComponent-0` :`bManualAttachment` true :`RelativeTransform` (`KismetMathLibrary.Conv_VectorToTransform` _returnvalue))))