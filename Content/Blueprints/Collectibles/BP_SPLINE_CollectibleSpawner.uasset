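; A spline-based spawner that lays out child actors, presumably collectibles, along a path.
; Its construction script adds them with manual attachment at world-space spline locations, looping from 0 to SpawnAmount.
; Each location samples spline time at Index / SpawnAmount without constant velocity, so spacing can vary with segment length.
; The event graph adds no runtime logic.
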(event `self.ReceiveBeginPlay`
  (`parent.ReceiveBeginPlay`))

(fn `UserConstructionScript`
  (`parent.UserConstructionScript`)
  (set `self.SpawnerComponent` (`self.Spline`))
  (for _index (range (+ (`self.SpawnAmount`) 1))
    (`AddComponent|NODE_AddChildActorComponent-1` :`bManualAttachment` true :`RelativeTransform` (`KismetMathLibrary.Conv_VectorToTransform` (`SplineComponent.GetLocationAtTime` (`self.Spline`) (/ (`KismetMathLibrary.Conv_IntToDouble` _index) (`KismetMathLibrary.Conv_IntToDouble` (`self.SpawnAmount`))) "World" false)))))