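; BP_tmpActor appears to be a scratch actor for testing screen-to-world deprojection with player controller 0.
; Each Tick deprojects a fixed screen point just beyond the top-left corner and moves Sphere a short distance along that ray, so it follows the view.
; It also prints the viewport size and deprojected world position as debug text.
; The X0 value decreases over time but does not drive the sphere.
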(event `self.ReceiveBeginPlay`)

(event `self.ReceiveTick`
  (params (DeltaSeconds :type "Float (single-precision)"))
  (bind _returnvalue (`GameplayStatics.GetPlayerController` 0))
  (bind (_worldposition _worlddirection) (`GameplayStatics.DeprojectScreenToWorld` _returnvalue (`KismetMathLibrary.MakeVector2D` -100.0 -100.0)))
  (bind (_sizex _sizey) (`PlayerController.GetViewportSize` _returnvalue))
  (set `self.X_0` (+ (* DeltaSeconds -100.0) (`self.X_0`)))
  (`KismetSystemLibrary.PrintString` (`KismetStringLibrary.Conv_Vector2dToString` (`KismetMathLibrary.MakeVector2D` (`KismetMathLibrary.Conv_IntToDouble` _sizex) (`KismetMathLibrary.Conv_IntToDouble` _sizey))) true true (struct :`R` 1.0 :`B` 0.050657 :`A` 1.0) 0.0)
  (`KismetSystemLibrary.PrintString` (`KismetStringLibrary.Conv_VectorToString` _worldposition) true true (struct :`R` 1.0 :`B` 0.895246 :`A` 1.0) 0.0)
  (`SceneComponent.K2_SetWorldLocation` (`self.Sphere`) (+ _worldposition (* _worlddirection 100.0)) false false))

(fn `UserConstructionScript`)