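; BeginplayColliderTest is a test actor with a box collider that reports when a SteikemannCharacter's capsule overlaps it.
; Half a second after BeginPlay, it saves the box extent, collapses it to zero and restores it with overlap updates on, forcing overlap re-evaluation.
; The box's begin-overlap event filters for the character's capsule component and prints the character's name.
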(event `self.ReceiveBeginPlay`
  (bind _box (`self.Box`))
  (`KismetSystemLibrary.Delay` 0.5)
  (bind _output_get (set `self.NewVar_0` (`BoxComponent.GetUnscaledBoxExtent` _box)))
  (`BoxComponent.SetBoxExtent` _box (0.0 0.0 0.0) true)
  (`BoxComponent.SetBoxExtent` _box _output_get true))

(event `self.Box.OnComponentBeginOverlap`
  (params (OverlappedComponent :type "PrimitiveComponent Object Reference") (OtherActor :type "Actor Object Reference") (OtherComp :type "PrimitiveComponent Object Reference") (OtherBodyIndex :type Integer) (bFromSweep :type Boolean) (SweepResult :type "HitResult Structure (by ref)"))
  (cast `CapsuleComponent` OtherComp)
  (bind _assteikemann_character (cast `SteikemannCharacter` OtherActor))
  (`KismetSystemLibrary.PrintString` (`KismetStringLibrary.Concat_StrStr` "Collided with: " (`KismetSystemLibrary.GetDisplayName` _assteikemann_character))))

(fn `UserConstructionScript`)