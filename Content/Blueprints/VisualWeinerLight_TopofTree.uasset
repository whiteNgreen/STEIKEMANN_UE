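; Point light actor, apparently for a treetop, that scales its brightness and volumetric scattering with the camera's vertical distance.
; BeginPlay caches both base values, and Tick multiplies them by PlayerDistanceCheck's exponential strength, computed from the height gap over FadeDistanceZ.
; FadeLight plays a timeline that scales base intensity, then sets a short lifespan to remove the actor.
; Tick keeps writing intensity during that fade.
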(event `self.ReceiveBeginPlay`
  (bind _pointlightcomponent (`self.PointLightComponent`))
  (set `self.Volumetric` (`LightComponentBase.VolumetricScatteringIntensity` _pointlightcomponent))
  (set `self.Intensity` (`LightComponentBase.Intensity` _pointlightcomponent)))

(event `self.ReceiveTick`
  (params (DeltaSeconds :type "Float (single-precision)"))
  (bind _pointlightcomponent (`self.PointLightComponent`))
  (bind _returnvalue (`PlayerDistanceCheck_Component.ExponentStrength` (`self.PlayerDistanceCheck_`) (/ (`KismetMathLibrary.Abs` (- (.z (`self.K2_GetActorLocation`)) (.z (`PlayerDistanceCheck_Component.GetPlayerCameraLocation` (`self.PlayerDistanceCheck_`))))) (`self.FadeDistanceZ`)) (`self.Top`) (`self.Bot`)))
  (`LightComponent.SetVolumetricScatteringIntensity` _pointlightcomponent (* (`self.Volumetric`) _returnvalue))
  (`LightComponent.SetIntensity` _pointlightcomponent (* (`self.Intensity`) _returnvalue)))

(event `Fade Light`
  (bind (_direction _intensitymultiplier) (`Timeline|LightFade` :!via `PlayFromStart`)
    (:`Update`
      (`LightComponent.SetIntensity` (`self.PointLightComponent`) (* _intensitymultiplier (`self.Intensity`))))
    (:`Finished`
      (`self.SetLifeSpan` 0.2))))

(fn `UserConstructionScript`)