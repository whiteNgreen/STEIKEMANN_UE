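; BP_EnemySpawner is an enemy spawner actor whose Blueprint contains only an editor visualization, with no spawn logic in its event graph.
; The construction script briefly draws two upward debug cones at the actor's location, using PitchRange X and Y as cone angles to show the pitch limits.
; A debug sphere for SpawnerMinRadius is left disconnected and never runs.
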(event `self.ReceiveBeginPlay`)

(event `self.ReceiveTick`
  (params (DeltaSeconds :type "Float (single-precision)")))

(fn `UserConstructionScript`
  (bind (_x _y) (`KismetMathLibrary.BreakVector2D` (`self.PitchRange`)))
  (bind _x_2 (`KismetMathLibrary.BreakVector2D` (`self.PitchRange`)))
  (`KismetSystemLibrary.DrawDebugConeInDegrees` (`self.K2_GetActorLocation`) (0.0 0.0 1.0) 2000.0 _x_2 _x_2 12 (struct :`R` 1.0 :`G` 1.0 :`B` 1.0 :`A` 1.0) 0.1 4.0)
  (`KismetSystemLibrary.DrawDebugConeInDegrees` (`self.K2_GetActorLocation`) (0.0 0.0 1.0) 2000.0 _y _y 12 (struct :`R` 0.898129 :`B` 1.0 :`A` 1.0) 0.1 4.0))