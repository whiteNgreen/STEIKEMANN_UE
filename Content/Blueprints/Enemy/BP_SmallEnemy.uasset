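; BP_SmallEnemy is a small enemy that serves as a grapple target and shows its targeting state through its mesh material.
; It caches the mesh's first material on BeginPlay, then swaps in highlight materials on the Targeted and InReach events.
; OutofReach and UnTargeted both restore the cached material.
; GetGrappledGameplayTag returns the GrappleTarget.Enemy tag to identify it as an enemy target.
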(event `self.ReceiveBeginPlay`
  (set `self.Base_Material` (`PrimitiveComponent.GetMaterial` (`self.Mesh`) 0)))

(event `GrappleTargetInterface.Targeted`
  (`PrimitiveComponent.SetMaterial` (`self.Mesh`) 0 "/Game/Materials/M_Grid_preset_035_Target.M_Grid_preset_035_Target"))

(event `GrappleTargetInterface.InReach`
  (`PrimitiveComponent.SetMaterial` (`self.Mesh`) 0 "/Game/Materials/M_Grid_preset_035_InReach.M_Grid_preset_035_InReach"))

(event `self.ReceiveTick`
  (params (DeltaSeconds :type "Float (single-precision)")))

(event `GrappleTargetInterface.OutofReach`
  (`PrimitiveComponent.SetMaterial` (`self.Mesh`) 0 (`self.Base_Material`) :!label _label))

(event `GrappleTargetInterface.UnTargeted`
  (goto _label))

(fn `GetGrappledGameplayTag`
  (returns (ReturnValue :type "GameplayTag Structure"))
  (return (struct :`TagName` "GrappleTarget.Enemy")))

(fn `UserConstructionScript`)